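; BP_SleepyChild is a side-quest NPC whose objective is picking up a teddy bear.
; TeddyTrigger, registered with the InteractableComponent, gates pickup by player overlap; interacting removes the teddy, re-enables talking and shows the alert marker.
; _Interact hides the player widget.
; Dialogue updates, teddy reveal, fish-bone reward and quest completion are present but disconnected, so never run here.
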(event `self.ReceiveBeginPlay`
  ;[1 1 1] IDK
  (bind _asbp_player_character (cast `/Game/Blueprints/Characters/BP_PlayerCharacter` (`GameplayStatics.GetPlayerCharacter` 0)))
  (set `self.Player` _asbp_player_character))

(event `self.InteractableComponent.OnInteract`
  (params (_playerCharacter :type "PlayerCharacter Object Reference"))
  (bind _questavailablemesh (`self.QuestAvailableMesh`))
  ;[1 1 1] Quest Objective
  (if (`self.CanPickupTeddy`)
    (`ActorComponent.K2_DestroyComponent` (`self.TeddyTrigger`))
    (`ActorComponent.K2_DestroyComponent` (`self.Teddy`))
    (set `self.CanNPCTalk` true)
    (`PrimitiveComponent.SetMaterial` _questavailablemesh 0 "/Game/Assets/Alert/M_Alert.M_Alert")
    (`SceneComponent.SetVisibility` _questavailablemesh true false)))

(event `self.TriggerBox.OnComponentEndOverlap`
  (params (OverlappedComponent :type "PrimitiveComponent Object Reference") (OtherActor :type "Actor Object Reference") (OtherComp :type "PrimitiveComponent Object Reference") (OtherBodyIndex :type Integer))
  ;[1 1 1] Walk out range
  (if (`self.ActorHasTag` OtherActor "Player")
    _))

(event `self.TeddyTrigger.OnComponentBeginOverlap`
  (params (OverlappedComponent :type "PrimitiveComponent Object Reference") (OtherActor :type "Actor Object Reference") (OtherComp :type "PrimitiveComponent Object Reference") (OtherBodyIndex :type Integer) (bFromSweep :type Boolean) (SweepResult :type "HitResult Structure (by ref)"))
  (cast `/Game/Blueprints/Characters/BP_PlayerCharacter` OtherActor)
  (set `self.CanPickupTeddy` true))

(event `self.TeddyTrigger.OnComponentEndOverlap`
  (params (OverlappedComponent :type "PrimitiveComponent Object Reference") (OtherActor :type "Actor Object Reference") (OtherComp :type "PrimitiveComponent Object Reference") (OtherBodyIndex :type Integer))
  (cast `/Game/Blueprints/Characters/BP_PlayerCharacter` OtherActor)
  (set `self.CanPickupTeddy` false))

(event `self.Receive_Interact`
  (`Widget.SetVisibility` (`PlayerCharacter.PlayerWidget` (`self.Player`)) "Hidden"))

(fn `UserConstructionScript`
  (`InteractableComponent.RegisterTriggerVolume` (`self.InteractableComponent`) (`self.TeddyTrigger`)))