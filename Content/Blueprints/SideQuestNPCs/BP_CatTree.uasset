(event `self.ReceiveBeginPlay`
  ;[0.1 0.1 0.1] Store BP_Playercharacter reference
  (bind _asbp_player_character (cast `/Game/Blueprints/Characters/Player/BP_PlayerCharacter` (`GameplayStatics.GetPlayerCharacter` 0)))
  (set `self.Player` _asbp_player_character)
  ;[0.1 0.1 0.1] Set objective complete on end of conversation
  (`DialogueSystemComponent.AttachQuestObjectiveToConversation` (`self.DialogueSystemComponent`) 0 (`self.Quest2Objective0`))
  (`DialogueSystemComponent.AttachQuestObjectiveToConversation` (`self.DialogueSystemComponent`) 1 (`self.Quest2Objective1`)))

(event `self.TomatoCollision.OnComponentHit`
  (params (HitComponent :type "PrimitiveComponent Object Reference") (OtherActor :type "Actor Object Reference") (OtherComp :type "PrimitiveComponent Object Reference") (NormalImpulse :type "Vector Structure") (Hit :type "HitResult Structure (by ref)"))
  (bind (_bblockinghit _binitialoverlap _time _distance _location _impactpoint _normal _impactnormal) (`GameplayStatics.BreakHitResult` Hit))
  (bind _treecat (`self.TreeCat`))
  ;[0.1 0.1 0.1] When branch hit by tomato, break, kid falls
  (if (`self.bCanBreakBranch`)
    (cast `/Game/Blueprints/Items/BP_Tomato` OtherActor)
    (set `InteractableComponent.bCanInteract` false (`self.InteractableComponent`))
    (set `self.bBranchBroken` true)
    (`self.ExplodeBranch` _impactpoint _impactnormal (`self.BranchExplodeStrength`))
    (`PrimitiveComponent.SetSimulatePhysics` _treecat true)
    (`SkeletalMeshComponent.PlayAnimation` _treecat "/Game/Assets/Catchild/NewModel/Animations/A_CatChild_Fall.A_CatChild_Fall" false)
    (set `InteractableComponent.bCanInteract` true (`self.InteractableComponent`))))

(event `self.InteractableComponent.OnPlayerExitInteractRange`
  (params (_playerCharacter :type "PlayerCharacter Object Reference"))
  ;[0.1 0.1 0.1] Disable dialogue when player walk out of the range
  (`DialogueSystemComponent.DisableDialogue` (`self.DialogueSystemComponent`) false))

(event `self.InteractableComponent.OnInteractSuccess`
  (params (_playerCharacter :type "PlayerCharacter Object Reference"))
  (bind _dialoguesystemcomponent (`self.DialogueSystemComponent`))
  ;[0.1 0.1 0.1] When player tries to talk with the kid
  (bind _playerwidget (`PlayerCharacter.PlayerWidget` _playerCharacter)
    (:`then`
      (`Widget.SetVisibility` _playerwidget "Hidden")
      (if (`|EnumInequality` (`QuestObjectiveComponent.ObjectiveState` (`self.Quest2Objective0`)) "Completed")
        (`DialogueSystemComponent.DialogueInteract` (`self.DialogueSystemComponent`) _playerCharacter 0 true) ; Gives out the quest
        (elif (`self.bBranchBroken`)
          (`DialogueSystemComponent.DialogueInteract` _dialoguesystemcomponent _playerCharacter 1 true) ; Thanks the player
          (else
            (`DialogueSystemComponent.DialogueInteract` _dialoguesystemcomponent _playerCharacter 2 true) ; Continue to ask for help
          ))))
    (:`else`)))

(event `self.DialogueSystemComponent.OnDialogueDisable`
  ;[0.1 0.1 0.1] Give player hud back
  (`Widget.SetVisibility` (`PlayerCharacter.PlayerWidget` (`self.Player`)) "Visible"))

(event `self.Quest2Objective0.OnObjectiveComplete`
  ;[0.1 0.1 0.1] After quest given, the branch become breakable
  (bind _ascatastrophe_main_game_mode (cast `CatastropheMainGameMode` (`GameplayStatics.GetGameMode`)))
  (`CatastropheMainGameMode.OnQuestObjectiveCompletion` _ascatastrophe_main_game_mode (`self.Quest2Objective0`) false)
  (set `self.bCanBreakBranch` true)
  (`PrimitiveComponent.SetRenderCustomDepth` (`self.DestructibleBranch`) true)
  (`PrimitiveComponent.SetMaterial` (`self.ObjectiveMarker`) 0 "/Game/Assets/Alert/ObjectiveMats/MI_objectives_Yellow.MI_Objectives_Yellow"))

(event `self.Quest2Objective1.OnObjectiveComplete`
  ;[0.1 0.1 0.1] When the player finishes the quest
  (bind _ascatastrophe_main_game_mode (cast `CatastropheMainGameMode` (`GameplayStatics.GetGameMode`)))
  (`CatastropheMainGameMode.OnQuestObjectiveCompletion` _ascatastrophe_main_game_mode (`self.Quest2Objective1`) false)
  (`|SpawnActorFromClass` "/Game/Blueprints/Interactables/BP_DisguisePickup.BP_DisguisePickup_C" (`KismetMathLibrary.Conv_VectorToTransform` (`SceneComponent.K2_GetComponentLocation` (`self.ItemSpawnLocation`))) "AlwaysSpawn" "OverrideRootScale" null null) ; Spawns the disguise pickup
  (`ActorComponent.K2_DestroyComponent` (`self.ObjectiveMarker`))
  (set `InteractableComponent.bCanInteract` false (`self.InteractableComponent`))
  (`KismetSystemLibrary.Delay` 2.0)
  (bind _returnvalue (`|CreateWidget` "/Game/Assets/UI/Widgets/Items/wbp_UnlockItem.WBP_UnlockItem_C"))
  (bind _output_get (set `self.ItemUnlockedWidget` _returnvalue))
  (`/Game/Assets/UI/Widgets/Items/wbp_UnlockItem.SetItemUnlock` _output_get "/Game/Assets/UI/AlphaIcons/T_Box_noBorder.T_Box_noBorder" "/Game/Blueprints/Gameplay/ItemInventory/BP_DisguiseSack.BP_DisguiseSack_C")
  (`UserWidget.AddToViewport` (`self.ItemUnlockedWidget`) 0)
  (`KismetSystemLibrary.Delay` 2.0)
  (`Widget.RemoveFromParent` (`self.ItemUnlockedWidget`)))

(event `self.Boxphysics collider.OnComponentBeginOverlap`
  (params (OverlappedComponent :type "PrimitiveComponent Object Reference") (OtherActor :type "Actor Object Reference") (OtherComp :type "PrimitiveComponent Object Reference") (OtherBodyIndex :type Integer) (bFromSweep :type Boolean) (SweepResult :type "HitResult Structure (by ref)"))
  ;[0.1 0.1 0.1] Stops the disguise pickup from falling
  (bind _asbp_disguise_pickup (cast `/Game/Blueprints/Interactables/BP_DisguisePickup` OtherActor))
  (`PrimitiveComponent.SetSimulatePhysics` (`ItemCrate.ItemMesh` _asbp_disguise_pickup) false))

(event `self.Boxphysics colliderCat.OnComponentBeginOverlap`
  (params (OverlappedComponent :type "PrimitiveComponent Object Reference") (OtherActor :type "Actor Object Reference") (OtherComp :type "PrimitiveComponent Object Reference") (OtherBodyIndex :type Integer) (bFromSweep :type Boolean) (SweepResult :type "HitResult Structure (by ref)"))
  ;[0.1 0.1 0.1] Stops cat falling
  (if (`ActorComponent.ComponentHasTag` OtherComp "Cat")
    (`PrimitiveComponent.SetSimulatePhysics` (`self.TreeCat`) false)))

(fn `ExplodeBranch`
  (params (HitLocation :type "Vector Structure") (ImpactNormal :type "Vector Structure") (Strength :type "Float (double-precision)"))
  (bind _destructiblebranch (`self.DestructibleBranch`))
  (`DestructibleComponent.ApplyDamage` _destructiblebranch 2.0 HitLocation (* ImpactNormal -1.0) Strength)
  (`PrimitiveComponent.SetCollisionEnabled` _destructiblebranch "NoCollision")
  (`PrimitiveComponent.SetRenderCustomDepth` _destructiblebranch false))

(fn `UserConstructionScript`)