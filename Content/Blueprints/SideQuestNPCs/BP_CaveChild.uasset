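; Side quest NPC Blueprint for a cave child whose quest involves a teddy.
; The FinishOldQuest event stops the NPC talking, hides its quest marker and reveals the teddy with its trigger, while FinishNewQuest destroys the marker.
; The player widget hides on interaction and returns when dialogue is disabled.
; Teddy interaction, registered through an InteractableComponent, only prints a placeholder, and the fish bone reward is unwired.
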(event `self.ReceiveBeginPlay`
  ;[1 1 1] IDK
  (bind _asplayer_character (cast `PlayerCharacter` (`GameplayStatics.GetPlayerCharacter` 0)))
  (set `self.Player` _asplayer_character))

(event `Receive_FinishOldQuest_1`
  ;[1 1 1] After starting dialogue
  (set `self.CanNPCTalk` false)
  (`SceneComponent.SetVisibility` (`self.QuestAvailableMesh`) false false)
  (`PrimitiveComponent.SetCollisionEnabled` (`self.TeddyTrigger`) "QueryAndPhysics")
  (`SceneComponent.SetVisibility` (`self.Teddy`) true false))

(event `self.InteractableComponent.OnInteract`
  (params (_playerCharacter :type "PlayerCharacter Object Reference"))
  ;[1 1 1] Quest Objective
  (`KismetSystemLibrary.PrintString` "Hello"))

(event `Receive_FinishNewQuest_1`
  ;[1 1 1] After Finishing dialogue
  (`ActorComponent.K2_DestroyComponent` (`self.QuestAvailableMesh`)))

(event `self.TriggerBox.OnComponentEndOverlap`
  (params (OverlappedComponent :type "PrimitiveComponent Object Reference") (OtherActor :type "Actor Object Reference") (OtherComp :type "PrimitiveComponent Object Reference") (OtherBodyIndex :type Integer))
  ;[1 1 1] Walk out range
  (if (`self.ActorHasTag` OtherActor "Player")
    _))

(event `self.Receive_Interact`
  (`Widget.SetVisibility` (`PlayerCharacter.PlayerWidget` (`self.Player`)) "Hidden"))

(event `Receive_DisableDialogue_1`
  (`Widget.SetVisibility` (`PlayerCharacter.PlayerWidget` (`self.Player`)) "Visible"))

(fn `UserConstructionScript`
  (`InteractableComponent.RegisterTriggerVolume` (`self.InteractableComponent`) (`self.TeddyTrigger`)))