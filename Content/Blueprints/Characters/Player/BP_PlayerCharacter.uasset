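; Player character Blueprint for the cat thief, tying together animation, UI and inventory.
; On BeginPlay it caches the animation Blueprint, adds quest-unlocked and required-item widgets, and initialises the inventory with four sack item types.
; Input toggles a lazily created pause menu, can open it on the quest journal section, and cycles items behind a delay gate.
; It also provides speed-reduction and randomised footstep functions; the sprint music logic is disconnected.
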(event `self.ReceiveBeginPlay`
  ;[1 1 1] Store the player animation blueprint
  (`parent.ReceiveBeginPlay`)
  (set `self.PlayerAnimationBP` (cast `/Game/Assets/MainCharacter/CatThief_Clothed/ABP_CatThief` (`SkeletalMeshComponent.GetAnimInstance` (`self.Mesh`)) :!pure true))
  (bind _returnvalue (`|CreateWidget` "/Game/Assets/UI/Widgets/Quests/WBP_QuestUnlocked.WBP_QuestUnlocked_C"))
  (bind _output_get (set `self.QuestWidget` _returnvalue))
  (`UserWidget.AddToViewport` _output_get 0)
  (bind _returnvalue_2 (`|CreateWidget` "/Game/Assets/UI/Widgets/WBP_ItemRequire.WBP_ItemRequire_C" (`GameplayStatics.GetPlayerController` 0)))
  (bind _output_get_2 (set `self.RequiredItemWidget` _returnvalue_2))
  (`UserWidget.AddToViewport` _output_get_2 0)
  (`InventoryComponent.InitialiseItemTypes` (`self.InventoryComponent`) (`|MakeArray` "/Game/Blueprints/Gameplay/ItemInventory/BP_TomatoSack.BP_TomatoSack_C" "/Game/Blueprints/Gameplay/ItemInventory/BP_DisguiseSack.BP_DisguiseSack_C" "/Game/Blueprints/Gameplay/ItemInventory/BP_YarnballSack.BP_YarnballSack_C" "/Game/Blueprints/Gameplay/ItemInventory/BP_CatnipBallSack.BP_CatnipBallSack_C" :!type "ItemSack Class Reference")))

(event `InputAction|Pause` :paused true
  (params (Key :type "Key Structure"))
  ;[1 1 1] Pause Game
  (:`Pressed`
    (if (`self.IsPaused`)
      (`self.UnPause Game`)
      (else
        (`self.Pause Game`)))))

(event `InputAction|QuestJournal` :paused true
  (params (Key :type "Key Structure"))
  ;[1 1 1] Opening Quest Journal
  (:`Pressed`
    (if (`self.IsPaused`)
      (`self.UnPause Game`)
      (else
        (`self.Pause Game`)
        (bind _aswbp_pause_menu (cast `/Game/Assets/UI/Widgets/WBP_PauseMenu` (`self.Pause Menu`)))
        (`WidgetSwitcher.SetActiveWidgetIndex` (`/Game/Assets/UI/Widgets/WBP_PauseMenu.Sections` _aswbp_pause_menu) 1)))))

(event `InputAction|PreviousItemSelect`
  (params (Key :type "Key Structure"))
  ;[1 1 1] Switching between items
  (:`Pressed`
    (if (`self.CanSwitchItem`)
      (`InventoryComponent.ChoosePreviousItem` (`self.InventoryComponent`))
      (set `self.CanSwitchItem` false)
      (`KismetSystemLibrary.Delay` (`self.ItemSwitchDelay`))
      (set `self.CanSwitchItem` true))))

(event `InputAction|NextItemSelect`
  (params (Key :type "Key Structure"))
  ;[1 1 1] Switching between items
  (:`Pressed`
    (if (`self.CanSwitchItem`)
      (`InventoryComponent.ChooseNextItem` (`self.InventoryComponent`))
      (set `self.CanSwitchItem` false)
      (`KismetSystemLibrary.Delay` (`self.ItemSwitchDelay`))
      (set `self.CanSwitchItem` true))))

(event `self.SprintMovementComponent.OnSprintBegin`
  ;[1 1 1] DEJAVU
)

(event `self.SprintMovementComponent.OnSprintEnd`
  ;[1 1 1] DEJAVU
)

(fn `LowerSpeed`
  (bind _charactermovement (`self.CharacterMovement`))
  (set `CharacterMovementComponent.MaxWalkSpeed` (* (`MovementComponent.GetMaxSpeed` _charactermovement) (- 1.0 (`self.MovementReduction`))) _charactermovement))

(fn `Pause Game`
  (`GameplayStatics.SetGamePaused` true)
  (`/Engine/EditorBlueprintResources/StandardMacros.IsValid` (`self.Pause Menu`)
    (:`Is Valid`
      _)
    (:`Is Not Valid`
      (bind _returnvalue (`|CreateWidget` "/Game/Assets/UI/Widgets/WBP_PauseMenu.WBP_PauseMenu_C" (`GameplayStatics.GetPlayerController` 0)))
      (bind _output_get (set `self.Pause Menu` _returnvalue))))
  (`UserWidget.AddToViewport` _output_get 100)
  (set `PlayerController.bShowMouseCursor` true (`GameplayStatics.GetPlayerController` 0))
  (set `self.IsPaused` true))

(fn `PlayFootStepSound`
  (`GameplayStatics.PlaySoundAtLocation` "/Game/Sound/Footsteps/Asphalt_Trainers_Walk_Slow/FOOTSTEP_Asphalt_Trainers_Walk_Slow_RR1_mono_Cue.FOOTSTEP_Asphalt_Trainers_Walk_Slow_RR1_mono_Cue" (`SceneComponent.K2_GetComponentLocation` (`self.Mesh`)) (struct) (`KismetMathLibrary.RandomFloatInRange` 0.1 0.2) (`KismetMathLibrary.RandomFloatInRange` 1.0 1.2) 0.0 "/Game/Assets/Attenuation/ATT_FootStep.ATT_FootStep" null null))

(fn `UnPause Game`
  (bind _returnvalue (`GameplayStatics.GetPlayerController` 0))
  (`Widget.RemoveFromParent` (`self.Pause Menu`))
  (`GameplayStatics.SetGamePaused` false)
  (`WidgetBlueprintLibrary.SetInputMode_GameOnly` _returnvalue)
  (set `PlayerController.bShowMouseCursor` false _returnvalue)
  (set `self.IsPaused` false))

(fn `UserConstructionScript`)