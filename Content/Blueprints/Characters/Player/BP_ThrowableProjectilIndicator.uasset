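; Blueprint that draws a trajectory indicator line for the player's throwable projectile from a supplied array of points.
; UpdateIndicaterLine rebuilds the spline in world space and divides its length into equal segments.
; Each mesh in SplineMeshes is stretched along one segment, with tangents clamped to segment length.
; The loop that creates collision-free mesh components is disconnected, so this graph only repositions existing entries.
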(event `self.K2_UpdateIndicaterLine`
  (params (_vectors :type "Array of Vector Structure (by ref)"))
  (bind _splinecomponent (`self.SplineComponent`))
  (bind _splinecomponent_2 (`self.SplineComponent`))
  (bind _splinecomponent_3 (`self.SplineComponent`))
  (`SplineComponent.ClearSplinePoints` _splinecomponent_2 true)
  (`SplineComponent.SetSplinePoints` _splinecomponent_2 _vectors "World" true)
  (set `self.SegmentLength` (/ (`SplineComponent.GetSplineLength` _splinecomponent_2) (`KismetMathLibrary.Conv_IntToDouble` (`self.NumberOfMeshSegments`))))
  (for (_array_element _array_index) (`self.SplineMeshes`)
    (bind _returnvalue (`KismetMathLibrary.Conv_IntToDouble` _array_index))
    (bind _returnvalue_2 (* (`self.SegmentLength`) _returnvalue))
    (bind _returnvalue_3 (* (+ _returnvalue 1.0) (`self.SegmentLength`)))
    (`SplineMeshComponent.SetStartAndEnd` _array_element (`SplineComponent.GetLocationAtDistanceAlongSpline` _splinecomponent_3 _returnvalue_2 "World") (`KismetMathLibrary.ClampVectorSize` (`SplineComponent.GetTangentAtDistanceAlongSpline` _splinecomponent_3 _returnvalue_2 "Local") 0.0 (`self.SegmentLength`)) (`SplineComponent.GetLocationAtDistanceAlongSpline` _splinecomponent _returnvalue_3 "World") (`KismetMathLibrary.ClampVectorSize` (`SplineComponent.GetTangentAtDistanceAlongSpline` _splinecomponent _returnvalue_3 "Local") 0.0 (`self.SegmentLength`)) true)))

(fn `UserConstructionScript`)