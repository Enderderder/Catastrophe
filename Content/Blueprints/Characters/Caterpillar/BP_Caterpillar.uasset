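; BP_Caterpillar is a caterpillar character that detects catching the player and can be slowed by boulders.
; Its CatchTriggerBox overlap only prints a debug message for actors tagged Player.
; Components tagged Boulder trigger a temporary speed reduction and their actor is destroyed.
; The slowdown subtracts from the walk speed cached at BeginPlay, then restores it after a Delay, so hits do not stack.
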(event `self.ReceiveBeginPlay`
  (set `self.MovementSpeed` (`CharacterMovementComponent.MaxWalkSpeed` (`self.CharacterMovement`))))

(event `self.CatchTriggerBox.OnComponentBeginOverlap`
  (params (OverlappedComponent :type "PrimitiveComponent Object Reference") (OtherActor :type "Actor Object Reference") (OtherComp :type "PrimitiveComponent Object Reference") (OtherBodyIndex :type Integer) (bFromSweep :type Boolean) (SweepResult :type "HitResult Structure (by ref)"))
  (`|ExecutionSequence`
    (:`then_0`
      (if (`self.ActorHasTag` OtherActor "Player")
        (`KismetSystemLibrary.PrintString` "CATERPIII: CAUGHT UUUUUUU UWU" true false (struct :`G` 0.66 :`B` 1.0 :`A` 1.0) 10.0)))
    (:`then_1`
      (if (`ActorComponent.ComponentHasTag` OtherComp "Boulder")
        (`self.Receive_ApplySpeedReduction` 500.0 2.0)
        (`self.K2_DestroyActor` OtherActor)))))

(event `self.Receive_ApplySpeedReduction`
  (params (_speed :type "Float (single-precision)") (_duration :type "Float (single-precision)"))
  (bind _charactermovement (`self.CharacterMovement`))
  (set `CharacterMovementComponent.MaxWalkSpeed` (- (`self.MovementSpeed`) _speed) _charactermovement)
  (`KismetSystemLibrary.Delay` _duration)
  (set `CharacterMovementComponent.MaxWalkSpeed` (`self.MovementSpeed`) _charactermovement))

(fn `UserConstructionScript`)