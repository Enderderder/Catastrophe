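; Larry NPC Blueprint that ties dialogue to two Quest 1 objectives, linked as the old and new quest on BeginPlay.
; Tick shows an alert or question-mark marker and enables talking while either objective is active.
; Overrides update the dialogue widget, hide the player HUD during interaction and stop dialogue when the player walks away.
; Finishing the old quest removes market collision, the new one grants fish bones, and completing Objective 3 destroys Larry.
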(event `self.ReceiveBeginPlay`
  ;[1 1 1] Linking Quests with Dialogue System
  (bind _asbp_player_character (cast `/Game/Blueprints/Characters/BP_PlayerCharacter` (`GameplayStatics.GetPlayerCharacter` 0)))
  (set `self.Player` _asbp_player_character)
  (for (_ _array_index) (`self.ConversationsList`)
    (switch `int` _array_index
      (:`0`
        (`self.SetConversationQuests` _array_index (`self.Quest1Objective0`) (`self.Quest1Objective3`))))))

(event `self.ReceiveTick`
  (params (DeltaSeconds :type "Float (single-precision)"))
  (bind _questavailablemesh (`self.QuestAvailableMesh`))
  (bind _questavailablemesh_2 (`self.QuestAvailableMesh`))
  ;[1 1 1] Activate/Deactivate quest available marker above head
  (if (or (`|EnumEquality` (`QuestObjectiveComponent.ObjectiveState` (`self.Quest1Objective0`)) "Active") (`|EnumEquality` (`QuestObjectiveComponent.ObjectiveState` (`self.Quest1Objective3`)) "Active"))
    (`SceneComponent.SetVisibility` _questavailablemesh true false)
    (if (== (`QuestObjectiveComponent.ObjectiveOrder` (`self.Quest1Objective0`)) 0)
      (`PrimitiveComponent.SetMaterial` _questavailablemesh_2 0 "/Game/Assets/Alert/M_Alert.M_Alert")
      (else
        (`PrimitiveComponent.SetMaterial` _questavailablemesh_2 0 "/Game/Assets/Questionmark/MI_QuestonMark.MI_QuestonMark")))
    (set `self.CanNPCTalk` true)
    (else
      (`SceneComponent.SetVisibility` _questavailablemesh false false))))

(event `self.Receive_UpdateWidget`
  (bind _dialoguewidget (`self.DialogueWidget`))
  ;[1 1 1] Updating Dialogue Widget
  (bind _aswbp_dialogue (cast `/Game/Assets/UI/Widgets/Dialogue/WBP_Dialogue` (`self.DialogueWidget`)))
  (`TextBlock.SetText` (`/Game/Assets/UI/Widgets/Dialogue/WBP_Dialogue.NPC_Text` _aswbp_dialogue) (`KismetTextLibrary.Conv_StringToText` (`self.CurrentNPCDialogueText`)))
  (`TextBlock.SetText` (`/Game/Assets/UI/Widgets/Dialogue/WBP_Dialogue.Player_Text` _aswbp_dialogue) (`KismetTextLibrary.Conv_StringToText` (`self.CurrentPlayerDialogueText`)))
  (bind _aswbp_dialogue_2 (cast `/Game/Assets/UI/Widgets/Dialogue/WBP_Dialogue` (`self.DialogueWidget`)))
  (bind _npc_icon (`/Game/Assets/UI/Widgets/Dialogue/WBP_Dialogue.NPC_Icon` _aswbp_dialogue_2))
  (`Image.SetBrush` _npc_icon (make `SlateBrush` (`Widget.GetDesiredSize` _npc_icon) (struct) (struct :`SpecifiedColor` (struct :`R` 1.0 :`G` 1.0 :`B` 1.0 :`A` 1.0) :`ColorUseRule` "UseColor_Specified") (`self.NPCIcon`)))
  (if (`self.IsNPCTalking`)
    (bind _aswbp_dialogue_3 (cast `/Game/Assets/UI/Widgets/Dialogue/WBP_Dialogue` _dialoguewidget))
    (`Widget.SetVisibility` (`/Game/Assets/UI/Widgets/Dialogue/WBP_Dialogue.NPC_Icon` _aswbp_dialogue_3) "Visible")
    (`Widget.SetVisibility` (`/Game/Assets/UI/Widgets/Dialogue/WBP_Dialogue.Player_Icon` _aswbp_dialogue_3) "Hidden")
    (else
      (bind _aswbp_dialogue_4 (cast `/Game/Assets/UI/Widgets/Dialogue/WBP_Dialogue` _dialoguewidget))
      (`Widget.SetVisibility` (`/Game/Assets/UI/Widgets/Dialogue/WBP_Dialogue.NPC_Icon` _aswbp_dialogue_4) "Hidden")
      (`Widget.SetVisibility` (`/Game/Assets/UI/Widgets/Dialogue/WBP_Dialogue.Player_Icon` _aswbp_dialogue_4) "Visible"))))

(event `self.TriggerBox.OnComponentEndOverlap`
  (params (OverlappedComponent :type "PrimitiveComponent Object Reference") (OtherActor :type "Actor Object Reference") (OtherComp :type "PrimitiveComponent Object Reference") (OtherBodyIndex :type Integer))
  ;[1 1 1] Stops Dialogue When Player Walks Away
  (cast `/Game/Blueprints/Characters/BP_PlayerCharacter` OtherActor)
  (`self.DisableDialogue`))

(event `self.Receive_FinishOldQuest`
  (set `self.CanNPCTalk` false)
  (`ActorComponent.K2_DestroyComponent` (`self.MarketCollision`))
  (`SceneComponent.SetVisibility` (`self.ObjectiveMesh (ChrisWayBecauseOtherOneIsBroken)`) false false))

(event `self.Receive_Interact`
  (`Widget.SetVisibility` (`PlayerCharacter.PlayerWidget` (`self.Player`)) "Hidden"))

(event `self.Receive_DisableDialogue`
  (`Widget.SetVisibility` (`PlayerCharacter.PlayerWidget` (`self.Player`)) "Visible"))

(event `self.Quest1Objective0.OnObjectiveActivate`)

(event `self.Quest1Objective0.OnObjectiveComplete`)

(event `self.Quest1Objective3.OnObjectiveActivate`)

(event `self.Quest1Objective3.OnObjectiveComplete`
  (`/Game/Assets/UI/Widgets/Quests/WBP_QuestUnlocked.QuestComplete` (`/Game/Blueprints/Characters/BP_PlayerCharacter.QuestWidget` (`self.Player`)) true)
  (`self.K2_DestroyActor`))

(event `self.Receive_FinishNewQuest`
  (set `PlayerCharacter.FishBonesAmount` (+ 10 (`PlayerCharacter.FishBonesAmount` (`self.Player`))) (`self.Player`)))

(fn `UserConstructionScript`)