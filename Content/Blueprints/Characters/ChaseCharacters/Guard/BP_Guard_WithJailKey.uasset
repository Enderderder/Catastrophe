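; Guard variant that carries the jail key, which the player takes to escape the jail as part of a quest objective.
; The construction script registers the key's trigger volume, and the key mesh renders to custom depth.
; Successful interaction completes the objective, removes the key and its marker, disables further interaction and unlocks the jail exit trigger.
; Objective completion notifies the main game mode without unlocking a new quest.
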(event `self.ReceiveBeginPlay`
  (`PrimitiveComponent.SetRenderCustomDepth` (`self.KeyMesh`) true))

(event `self.KeyInteractableComponent.OnInteractSuccess`
  (params (_playerCharacter :type "PlayerCharacter Object Reference"))
  ;[1 1 1] When key is picked up
  (`QuestObjectiveComponent.CompleteObjective` (`self.Quest0Objective2`))
  (`ActorComponent.K2_DestroyComponent` (`self.KeyMesh`))
  (set `InteractableComponent.bCanInteract` false (`self.KeyInteractableComponent`))
  (`ActorComponent.K2_DestroyComponent` (`self.ObjectiveMarker`))
  (`/Game/Blueprints/Interactables/Prison/Doors/BP_LockedDoor.UnlockDoor` (`self.JailExitTrigger`)))

(event `self.Quest0Objective2.OnObjectiveComplete`
  ;[1 1 1] When objective is completed
  (bind _ascatastrophe_main_game_mode (cast `CatastropheMainGameMode` (`GameplayStatics.GetGameMode`)))
  (`CatastropheMainGameMode.OnQuestObjectiveCompletion` _ascatastrophe_main_game_mode (`self.Quest0Objective2`) false))

(fn `UserConstructionScript`
  (`parent.UserConstructionScript`)
  ;[1 1 1] Register key interaction trigger
  (`InteractableComponent.RegisterTriggerVolume` (`self.KeyInteractableComponent`) (`self.KeyTrigger`)))