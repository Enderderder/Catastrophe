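; BP_Caterpillar is the caterpillar chase character for the cave gameplay sequence.
; It binds to the main game mode's cave begin, end and reset events; begin and end toggle the chase flag, while reset is empty.
; During the chase, Tick traces downward and aligns the mesh to the ground normal.
; A speed reduction event temporarily lowers walk speed, then restores the value cached at BeginPlay.
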(event `OnCaveGameplayBegin`
  (set `self.bChaseActive` true))

(event `OnCaveGameplayEnd`
  (set `self.bChaseActive` false))

(event `OnCaveGameplayReset`)

(event `self.ReceiveBeginPlay`
  ;[0.1 0.1 0.1] Stores the default movement speed
  (set `self.MovementSpeed` (`CharacterMovementComponent.MaxWalkSpeed` (`self.CharacterMovement`)))
  (bind _asbp_catastrophe_main_game_mode (cast `/Game/Blueprints/Gameplay/Gamemodes/BP_CatastropheMainGameMode` (`GameplayStatics.GetGameMode`)))
  (add `CatastropheMainGameMode.OnCaveGameplayBegin` _asbp_catastrophe_main_game_mode (delegate `OnCaveGameplayBegin`))
  (add `CatastropheMainGameMode.OnCaveGameplayEnd` _asbp_catastrophe_main_game_mode (delegate `OnCaveGameplayEnd`))
  (add `CatastropheMainGameMode.OnCaveGameplayReset` _asbp_catastrophe_main_game_mode (delegate `OnCaveGameplayReset`)))

(event `self.ReceiveTick`
  (params (DeltaSeconds :type "Float (single-precision)"))
  (bind (_returnvalue_x _returnvalue_y _returnvalue_z) (`KismetMathLibrary.BreakVector` (`self.K2_GetActorLocation`)))
  ;[0.1 0.1 0.1] During the cave chase, make sure the caterpillar is always up right against the ground
  (if (`self.bChaseActive`)
    (bind (_outhit _returnvalue) (`KismetSystemLibrary.LineTraceSingle` :`Start` (`KismetMathLibrary.MakeVector` _returnvalue_x _returnvalue_y _returnvalue_z) :`End` (`KismetMathLibrary.MakeVector` _returnvalue_x _returnvalue_y (- _returnvalue_z 1000.0)) :`TraceChannel` "TraceTypeQuery1" :`bTraceComplex` true :`DrawTime` 0.0))
    (if _returnvalue
      (`SceneComponent.K2_SetWorldRotation` (`self.Mesh`) (`KismetMathLibrary.MakeRotFromZX` (`.Normal` (`GameplayStatics.BreakHitResult` _outhit)) (`self.GetActorForwardVector`)) false false))))

(event `self.Receive_ApplySpeedReduction`
  (params (_speed :type "Float (single-precision)") (_duration :type "Float (single-precision)"))
  (bind _charactermovement (`self.CharacterMovement`))
  ;[0.1 0.1 0.1] Applies a speed reduction with duration
  (set `CharacterMovementComponent.MaxWalkSpeed` (- (`self.MovementSpeed`) _speed) _charactermovement)
  (`KismetSystemLibrary.Delay` _duration)
  (set `CharacterMovementComponent.MaxWalkSpeed` (`self.MovementSpeed`) _charactermovement))

(fn `UserConstructionScript`)