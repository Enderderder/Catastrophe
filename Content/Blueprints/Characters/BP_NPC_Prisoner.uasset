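; Prisoner NPC that offers a quest through dialogue and pays fishbone rewards to the player.
; On BeginPlay it binds QuestObjective0 to its first conversation and marks the owning quest available.
; Dialogue events refresh text and speaker icons, toggle the player HUD, and end the conversation when the player leaves the trigger box.
; Quest events add rewards, notify the quest widget on activation, and hide the availability marker on start or completion.
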(event `self.ReceiveBeginPlay`
  (bind _questobjective0 (`self.QuestObjective0`))
  ;[1 1 1] Linking Quests with Dialogue System
  (bind _asbp_player_character (cast `/Game/Blueprints/Characters/BP_PlayerCharacter` (`GameplayStatics.GetPlayerCharacter` 0)))
  (set `self.Player` _asbp_player_character)
  (for (_ _array_index) (`self.ConversationsList`)
    (switch `int` _array_index
      (:`0`
        (`self.SetConversationQuests` _array_index _questobjective0)
        (`Quest.SetQuestState` (`QuestObjectiveComponent.OwningQuest` _questobjective0) "Avaliable")))))

(event `self.Receive_UpdateWidget`
  (bind _dialoguewidget (`self.DialogueWidget`))
  ;[1 1 1] Updating Dialogue Widget
  (bind _aswbp_dialogue (cast `/Game/Assets/UI/Widgets/Dialogue/WBP_Dialogue` (`self.DialogueWidget`)))
  (`TextBlock.SetText` (`/Game/Assets/UI/Widgets/Dialogue/WBP_Dialogue.NPC_Text` _aswbp_dialogue) (`KismetTextLibrary.Conv_StringToText` (`self.CurrentNPCDialogueText`)))
  (`TextBlock.SetText` (`/Game/Assets/UI/Widgets/Dialogue/WBP_Dialogue.Player_Text` _aswbp_dialogue) (`KismetTextLibrary.Conv_StringToText` (`self.CurrentPlayerDialogueText`)))
  (bind _aswbp_dialogue_2 (cast `/Game/Assets/UI/Widgets/Dialogue/WBP_Dialogue` (`self.DialogueWidget`)))
  (bind _npc_icon (`/Game/Assets/UI/Widgets/Dialogue/WBP_Dialogue.NPC_Icon` _aswbp_dialogue_2))
  (`Image.SetBrush` _npc_icon (make `SlateBrush` (`Widget.GetDesiredSize` _npc_icon) (struct) (struct :`SpecifiedColor` (struct :`R` 1.0 :`G` 1.0 :`B` 1.0 :`A` 1.0) :`ColorUseRule` "UseColor_Specified") (`self.NPCIcon`)))
  (if (`self.IsNPCTalking`)
    (bind _aswbp_dialogue_3 (cast `/Game/Assets/UI/Widgets/Dialogue/WBP_Dialogue` _dialoguewidget))
    (`Widget.SetVisibility` (`/Game/Assets/UI/Widgets/Dialogue/WBP_Dialogue.NPC_Icon` _aswbp_dialogue_3) "Visible")
    (`Widget.SetVisibility` (`/Game/Assets/UI/Widgets/Dialogue/WBP_Dialogue.Player_Icon` _aswbp_dialogue_3) "Hidden")
    (else
      (bind _aswbp_dialogue_4 (cast `/Game/Assets/UI/Widgets/Dialogue/WBP_Dialogue` _dialoguewidget))
      (`Widget.SetVisibility` (`/Game/Assets/UI/Widgets/Dialogue/WBP_Dialogue.NPC_Icon` _aswbp_dialogue_4) "Hidden")
      (`Widget.SetVisibility` (`/Game/Assets/UI/Widgets/Dialogue/WBP_Dialogue.Player_Icon` _aswbp_dialogue_4) "Visible"))))

(event `self.TriggerBox.OnComponentEndOverlap`
  (params (OverlappedComponent :type "PrimitiveComponent Object Reference") (OtherActor :type "Actor Object Reference") (OtherComp :type "PrimitiveComponent Object Reference") (OtherBodyIndex :type Integer))
  ;[1 1 1] Stops Dialogue When Player Walks Away
  (cast `/Game/Blueprints/Characters/BP_PlayerCharacter` OtherActor)
  (`self.DisableDialogue`))

(event `self.Receive_FinishOldQuest`
  ;[1 1 1] OnFinish of OldQuest
  (bind _returnvalue (`self.GetCurrentFishboneReward_OldQuest`))
  (set `PlayerCharacter.FishBonesAmount` (+ _returnvalue (`PlayerCharacter.FishBonesAmount` (`self.Player`))) (`self.Player`)))

(event `self.Receive_FinishNewQuest`
  ;[1 1 1] OnFinish of NewQuest
  (bind _returnvalue (`self.GetCurrentFishboneReward_NewQuest`))
  (set `PlayerCharacter.FishBonesAmount` (+ _returnvalue (`PlayerCharacter.FishBonesAmount` (`self.Player`))) (`self.Player`)))

(event `self.QuestObjective0.OnObjectiveActivate`
  ;[1 1 1] Printing to screen when Quests activated/completed
  (`/Game/Assets/UI/Widgets/Quests/WBP_QuestUnlocked.OnQuestUnlocked` (`/Game/Blueprints/Characters/BP_PlayerCharacter.QuestWidget` (`self.Player`))))

(event `self.QuestObjective0.OnObjectiveComplete`
  ;[1 1 1] Printing to screen when Quests activated/completed
  (`SceneComponent.SetVisibility` (`self.ObjectiveAvailableMarker`) false false))

(event `self.Receive_Interact`
  (`SceneComponent.SetVisibility` (`self.TextRender`) false false)
  (`Widget.SetVisibility` (`PlayerCharacter.PlayerWidget` (`self.Player`)) "Hidden"))

(event `self.Receive_DisableDialogue`
  (`Widget.SetVisibility` (`PlayerCharacter.PlayerWidget` (`self.Player`)) "Visible"))

(event `self.Receive_StartNewQuest`
  (`SceneComponent.SetVisibility` (`self.ObjectiveAvailableMarker`) false false))

(fn `UserConstructionScript`)