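; Cave kid NPC that starts the cave gameplay once the player finishes talking to it.
; When the conversation ends, it plays a throw animation, attaches a catnip effect to the player and calls the game mode to start.
; Game mode cave events toggle talk availability and CaterpillarGate collision, off on begin and restored on reset, while the end handler is empty.
; Leaving the trigger box disables dialogue.
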(event `OnCaveGameplayBegin`
  (set `self.CanTalk` false)
  (`PrimitiveComponent.SetCollisionEnabled` (`self.CaterpillarGate`) "NoCollision"))

(event `OnCaveGameplayEnd`)

(event `OnCaveGameplayReset`
  (set `self.CanTalk` true)
  (`PrimitiveComponent.SetCollisionEnabled` (`self.CaterpillarGate`) "QueryAndPhysics"))

(event `self.ReceiveBeginPlay`
  (bind _asbp_catastrophe_main_game_mode (cast `/Game/Blueprints/Gameplay/Gamemodes/BP_CatastropheMainGameMode` (`GameplayStatics.GetGameMode`)))
  (add `CatastropheMainGameMode.OnCaveGameplayBegin` _asbp_catastrophe_main_game_mode (delegate `OnCaveGameplayBegin`))
  (add `CatastropheMainGameMode.OnCaveGameplayEnd` _asbp_catastrophe_main_game_mode (delegate `OnCaveGameplayEnd`))
  (add `CatastropheMainGameMode.OnCaveGameplayReset` _asbp_catastrophe_main_game_mode (delegate `OnCaveGameplayReset`)))

(event `self.Receive_Interact`
  ;[1 1 1] When the player interacts with the npc, start dialogue
  (`DialogueSystemComponent.DialogueInteract` (`self.DialogueSystemComponent`) null 0 (`self.CanTalk`)))

(event `self.DialogueSystemComponent.OnConversationEnd`
  (params (ConversationIndex :type Integer))
  ;[1 1 1] When the player finish the talk, start the cave gameplay
  (`DialogueSystemComponent.DisableDialogue` (`self.DialogueSystemComponent`) false)
  (`SkeletalMeshComponent.PlayAnimation` (`self.Demi`) "/Game/Assets/Kitsets/Mousehut/A_Demi_Throw__1_.A_Demi_Throw__1_" false)
  (`KismetSystemLibrary.Delay` 0.3)
  (`GameplayStatics.SpawnEmitterAttached` "/Game/VFX/Catnip/P_Catnip.P_Catnip" (`Character.Mesh` (`GameplayStatics.GetPlayerCharacter` 0)) "Catnip")
  (bind _asbp_catastrophe_main_game_mode (cast `/Game/Blueprints/Gameplay/Gamemodes/BP_CatastropheMainGameMode` (`GameplayStatics.GetGameMode`)))
  (`CatastropheMainGameMode.StartCaveGameplay` _asbp_catastrophe_main_game_mode))

(event `self.TriggerBox.OnComponentEndOverlap`
  (params (OverlappedComponent :type "PrimitiveComponent Object Reference") (OtherActor :type "Actor Object Reference") (OtherComp :type "PrimitiveComponent Object Reference") (OtherBodyIndex :type Integer))
  (if (`self.ActorHasTag` OtherActor "Player")
    (`DialogueSystemComponent.DisableDialogue` (`self.DialogueSystemComponent`) false)))

(fn `UserConstructionScript`)