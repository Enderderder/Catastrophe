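; Gandalf NPC that talks to the player and, once passage is allowed, walks away to a set location.
; Interacting starts one of two conversations based on the AllowPassage flag, and leaving the trigger disables dialogue.
; Ending the passage conversation disables interaction, then writes a new NPC state and rotation-relative walk target to the Blackboard.
; It reuses the wandering cat AI controller, initialized on BeginPlay with wander settings.
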(event `self.ReceiveBeginPlay`
  (bind _asbp_player_character (cast `/Game/Blueprints/Characters/Player/BP_PlayerCharacter` (`GameplayStatics.GetPlayerCharacter` 0)))
  (set `self.Player` _asbp_player_character)
  ;[1 1 1] Initialize AI Controller Variables
  (bind _asaic_npc_wandering_cat (cast `/Game/Blueprints/Characters/NPCs/WanderingNPCs/CatNPC/AIC_NPC_WanderingCat` (`AIBlueprintHelperLibrary.GetAIController` self)))
  (`/Game/Blueprints/Characters/NPCs/WanderingNPCs/CatNPC/AIC_NPC_WanderingCat.Initialize` _asaic_npc_wandering_cat (`self.NPCState`) (* (`self.WalkToLocation`) (`SceneComponent.K2_GetComponentLocation` (`self.CapsuleComponent`))) (`self.MinWanderDistance`) (`self.MaxWanderDistance`) (`self.MinWanderPauseTime`) (`self.MaxWanderPauseTime`)))

(event `self.InteractableComponent.OnInteractSuccess`
  (params (_playerCharacter :type "PlayerCharacter Object Reference"))
  (if (`self.bAllowPassage`)
    (`DialogueSystemComponent.DialogueInteract` (`self.DialogueSystemComponent`) _playerCharacter 1 true)
    (else
      (`DialogueSystemComponent.DialogueInteract` (`self.DialogueSystemComponent`) _playerCharacter 0 true))))

(event `self.InteractionTrigger.OnComponentEndOverlap`
  (params (OverlappedComponent :type "PrimitiveComponent Object Reference") (OtherActor :type "Actor Object Reference") (OtherComp :type "PrimitiveComponent Object Reference") (OtherBodyIndex :type Integer))
  (`DialogueSystemComponent.DisableDialogue` (`self.DialogueSystemComponent`) (`self.ActorHasTag` OtherActor "Player")))

(event `self.DialogueSystemComponent.OnConversationEnd`
  (params (ConversationIndex :type Integer))
  (if (== ConversationIndex 1)
    (`self.AllowPassage`)))

(fn `AllowPassage`
  (set `InteractableComponent.bCanInteract` false (`self.InteractableComponent`))
  (`self.UpdateNPCState` "NewEnumerator2")
  (`BlackboardComponent.SetValueAsVector` (`AIBlueprintHelperLibrary.GetBlackboard` self) (`KismetStringLibrary.Conv_StringToName` "WalkToLocation") (+ (`self.K2_GetActorLocation`) (`KismetMathLibrary.GreaterGreater_VectorRotator` (`self.WalkToLocation`) (`self.K2_GetActorRotation`)))))

(fn `UpdateNPCState`
  (params (NPCState :type "/Game/Blueprints/Characters/NPCs/WanderingNPCs/ENPCState Enum" :default "NewEnumerator0"))
  (bind _output_get (set `self.NPCState` NPCState))
  (`BlackboardComponent.SetValueAsEnum` (`AIBlueprintHelperLibrary.GetBlackboard` self) (`KismetStringLibrary.Conv_StringToName` "NPCState") _output_get))

(fn `UserConstructionScript`
  (`InteractableComponent.RegisterTriggerVolume` (`self.InteractableComponent`) (`self.InteractionTrigger`)))