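; BP_NPC_Prisoner is a prisoner NPC that the player talks to as part of a quest.
; On BeginPlay it attaches QuestObjective0 to its first conversation, which interacting starts with the player HUD hidden while the objective is incomplete.
; Completing the objective hides its marker, notifies CatastropheMainGameMode and disables further interaction.
; Walking out of range cancels the dialogue, and the HUD returns when dialogue is disabled.
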(event `self.ReceiveBeginPlay`
  ;[0.1 0.1 0.1] Store BP_PlayerCharacter reference
  (bind _asbp_player_character (cast `/Game/Blueprints/Characters/Player/BP_PlayerCharacter` (`GameplayStatics.GetPlayerCharacter` 0)))
  (set `self.Player` _asbp_player_character)
  ;[0.1 0.1 0.1] Linking Quests with Dialogue System
  (`DialogueSystemComponent.AttachQuestObjectiveToConversation` (`self.DialogueSystemComponent`) 0 (`self.QuestObjective0`)))

(event `self.InteractableComponent.OnInteractSuccess`
  (params (_playerCharacter :type "PlayerCharacter Object Reference"))
  ;[0.1 0.1 0.1] Gives out the quest
  (if (`|EnumInequality` (`QuestObjectiveComponent.ObjectiveState` (`self.QuestObjective0`)) "Completed")
    (bind _asbp_player_character (cast `/Game/Blueprints/Characters/Player/BP_PlayerCharacter` _playerCharacter))
    (bind _playerwidget (`PlayerCharacter.PlayerWidget` _asbp_player_character)
      (:`then`
        (`Widget.SetVisibility` _playerwidget "Hidden")
        (`DialogueSystemComponent.DialogueInteract` (`self.DialogueSystemComponent`) _playerCharacter 0 true) ; Gives out the quest
      )
      (:`else`))))

(event `self.QuestObjective0.OnObjectiveComplete`
  ;[0.1 0.1 0.1] Make objective marker disappear after talk
  (`SceneComponent.SetVisibility` (`self.ObjectiveAvailableMarker`) false false)
  (bind _ascatastrophe_main_game_mode (cast `CatastropheMainGameMode` (`GameplayStatics.GetGameMode`)))
  (`CatastropheMainGameMode.OnQuestObjectiveCompletion` _ascatastrophe_main_game_mode (`self.QuestObjective0`) false)
  (set `InteractableComponent.bCanInteract` false (`self.InteractableComponent`)))

(event `self.DialogueSystemComponent.OnDialogueDisable`
  ;[0.1 0.1 0.1] Gives hud back to the player after conversation
  (bind _player (`self.Player`)
    (:`then`
      (bind _playerwidget (`PlayerCharacter.PlayerWidget` _player)
        (:`then`
          (`Widget.SetVisibility` _playerwidget "Visible"))
        (:`else`)))
    (:`else`)))

(event `self.InteractableComponent.OnPlayerExitInteractRange`
  (params (_playerCharacter :type "PlayerCharacter Object Reference"))
  ;[0.1 0.1 0.1] Stops Dialogue When Player Walks Away
  (`DialogueSystemComponent.DisableDialogue` (`self.DialogueSystemComponent`) false))

(fn `UserConstructionScript`)