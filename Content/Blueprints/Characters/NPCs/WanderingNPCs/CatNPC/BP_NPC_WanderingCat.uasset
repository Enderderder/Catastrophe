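; Wandering cat NPC that the player can interact with to hear a randomly chosen conversation.
; On BeginPlay it picks a random skin and passes wander settings to its AI controller.
; InteractableComponent events toggle a camera-facing speech bubble and drive DialogueSystem, turning the cat toward the player and pausing wandering through Blackboard bools.
; Leaving interact range disables dialogue and re-enables wandering, so the next interaction rerolls the conversation.
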(event `self.ReceiveBeginPlay`
  (bind _skins (`self.Skins`))
  ;[1 1 1] OnBeginPlay
  ;;[1 1 1] Randomly choose a skin
  (`PrimitiveComponent.SetMaterial` (`self.Mesh`) 0 (`|GetArrayItem` _skins (`KismetMathLibrary.RandomIntegerInRange` 0 (- (`KismetArrayLibrary.Array_Length` _skins) 1))))
  ;;[1 1 1] Initialise AI Variables
  (bind _asaic_npc_wandering_cat (cast `/Game/Blueprints/Characters/NPCs/WanderingNPCs/CatNPC/AIC_NPC_WanderingCat` (`AIBlueprintHelperLibrary.GetAIController` self)))
  (`/Game/Blueprints/Characters/NPCs/WanderingNPCs/CatNPC/AIC_NPC_WanderingCat.Initialize` _asaic_npc_wandering_cat (`self.NPCState`) (0.0 0.0 0.0) (`self.MinWanderDistance`) (`self.MaxWanderDistance`) (`self.MinWanderPauseTime`) (`self.MaxWanderPauseTime`)))

(event `self.InteractableComponent.OnInteractSuccess`
  (params (_playerCharacter :type "PlayerCharacter Object Reference"))
  (bind (_returnvalue_x _returnvalue_y) (`KismetMathLibrary.BreakVector` (`self.K2_GetActorLocation` _playerCharacter)))
  (bind (_returnvalue_x_2 _returnvalue_y_2 _returnvalue_z) (`KismetMathLibrary.BreakVector` (`self.K2_GetActorLocation`)))
  (bind _returnvalue (`AIBlueprintHelperLibrary.GetBlackboard` null))
  ;[1 1 1] On Interaction Use Dialogue
  (`MovementComponent.StopMovementImmediately` (`self.CharacterMovement`))
  (`BlackboardComponent.SetValueAsBool` _returnvalue (`KismetStringLibrary.Conv_StringToName` "bCanWander") false)
  (`BlackboardComponent.SetValueAsBool` _returnvalue (`KismetStringLibrary.Conv_StringToName` "bIsWandering") false)
  (`SceneComponent.K2_SetWorldRotation` (`self.CapsuleComponent`) (`KismetMathLibrary.FindLookAtRotation` (`self.K2_GetActorLocation`) (`KismetMathLibrary.MakeVector` _returnvalue_x _returnvalue_y _returnvalue_z)) false false)
  (if (not (`self.bIsTalking`))
    (`self.ChooseRandomConversation`)
    (set `self.bIsTalking` true))
  (`DialogueSystemComponent.DialogueInteract` (`self.DialogueSystem`) null (`self.RandomConversationIndex`) true))

(event `self.InteractableComponent.OnPlayerEnterInteractRange`
  (params (_playerCharacter :type "PlayerCharacter Object Reference"))
  ;[0.1 0.1 0.1] Turn on speech bubble if player get close
  (`SceneComponent.SetVisibility` (`self.SpeechBubble`) true false))

(event `self.InteractableComponent.OnPlayerExitInteractRange`
  (params (_playerCharacter :type "PlayerCharacter Object Reference"))
  ;[0.1 0.1 0.1] After player walks away
  (`DialogueSystemComponent.DisableDialogue` (`self.DialogueSystem`) false)
  (`self.ReturnToWandering`)
  (`SceneComponent.SetVisibility` (`self.SpeechBubble`) false false))

(event `ReturnToWandering`
  ;[1 1 1] Return to wander
  (`BlackboardComponent.SetValueAsBool` (`AIBlueprintHelperLibrary.GetBlackboard` null) (`KismetStringLibrary.Conv_StringToName` "bCanWander") true)
  (set `self.bIsTalking` false))

(event `self.ReceiveTick`
  (params (DeltaSeconds :type "Float (single-precision)"))
  (bind _bubbleroot (`self.BubbleRoot`))
  (bind (_returnvalue_roll _returnvalue_pitch) (`KismetMathLibrary.BreakRotator` (`SceneComponent.K2_GetComponentRotation` _bubbleroot)))
  (bind (_returnvalue_roll_2 _returnvalue_pitch_2 _returnvalue_yaw) (`KismetMathLibrary.BreakRotator` (`KismetMathLibrary.FindLookAtRotation` (`SceneComponent.K2_GetComponentLocation` _bubbleroot) (`PlayerCameraManager.GetCameraLocation` (`GameplayStatics.GetPlayerCameraManager` 0)))))
  ;[0.1 0.1 0.1] If speech bubble is visible, rotate towards the camera
  (if (`SceneComponent.IsVisible` (`self.SpeechBubble`))
    (`SceneComponent.K2_SetWorldRotation` (`self.BubbleRoot`) (`KismetMathLibrary.MakeRotator` _returnvalue_roll _returnvalue_pitch _returnvalue_yaw) false false)))

(fn `ChooseRandomConversation`
  (set `self.RandomConversationIndex` (`KismetMathLibrary.RandomIntegerInRange` 0 (- (`KismetArrayLibrary.Array_Length` (`DialogueSystemComponent.Conversations` (`self.DialogueSystem`))) 1))))

(fn `UserConstructionScript`
  (`InteractableComponent.RegisterTriggerVolume` (`self.InteractableComponent`) (`self.InteractionTrigger`)))