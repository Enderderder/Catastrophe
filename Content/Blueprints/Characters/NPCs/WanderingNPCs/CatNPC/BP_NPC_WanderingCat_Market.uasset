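; Market variant of the wandering cat NPC that gets launched upward when it touches a guard.
; An overlap on its FlyTrigger filters for a Guard actor and a component tagged "Body".
; It then applies a velocity-change impulse along the cat's up vector, scaled by FlyStrength, and immediately calls StopMovementImmediately on the movement component.
; The construction script only runs the parent's.
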(event `self.FlyTrigger.OnComponentBeginOverlap`
  (params (OverlappedComponent :type "PrimitiveComponent Object Reference") (OtherActor :type "Actor Object Reference") (OtherComp :type "PrimitiveComponent Object Reference") (OtherBodyIndex :type Integer) (bFromSweep :type Boolean) (SweepResult :type "HitResult Structure (by ref)"))
  (bind _charactermovement (`self.CharacterMovement`))
  (cast `Guard` OtherActor) ; If its a guard
  (if (`ActorComponent.ComponentHasTag` OtherComp "Body")
    ;[0.1 0.1 0.1] Go fly when touch a guard
    (`CharacterMovementComponent.AddImpulse` _charactermovement (* (`self.GetActorUpVector`) (`self.FlyStrength`)) true)
    (`MovementComponent.StopMovementImmediately` _charactermovement)))

(fn `UserConstructionScript`
  (`parent.UserConstructionScript`))