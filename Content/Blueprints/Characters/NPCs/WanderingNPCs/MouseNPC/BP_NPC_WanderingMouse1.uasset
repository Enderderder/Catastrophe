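; Wandering mouse NPC that stops to talk when the player interacts with it.
; Interaction halts movement, clears the wander Blackboard flags, turns the capsule toward the player and starts dialogue through DialogueSystemComponent.
; The conversation is picked at random on first interaction and reused afterwards, since IsTalking is never reset here.
; Conversation end or the player leaving InteractTrigger re-enables wandering; leaving also disables dialogue.
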(event `self.InteractableComponent.OnInteractSuccess`
  (params (_playerCharacter :type "PlayerCharacter Object Reference"))
  (bind _returnvalue (`AIBlueprintHelperLibrary.GetBlackboard` null))
  (bind (_returnvalue_x _returnvalue_y _returnvalue_z) (`KismetMathLibrary.BreakVector` (`self.K2_GetActorLocation`)))
  (bind (_returnvalue_x_2 _returnvalue_y_2) (`KismetMathLibrary.BreakVector` (`self.K2_GetActorLocation` _playerCharacter)))
  (`MovementComponent.StopMovementImmediately` (`self.CharacterMovement`))
  (`BlackboardComponent.SetValueAsBool` _returnvalue (`KismetStringLibrary.Conv_StringToName` "bCanWander") false)
  (`BlackboardComponent.SetValueAsBool` _returnvalue (`KismetStringLibrary.Conv_StringToName` "bIsWandering") false)
  (`SceneComponent.K2_SetWorldRotation` (`self.CapsuleComponent`) (`KismetMathLibrary.FindLookAtRotation` (`self.K2_GetActorLocation`) (`KismetMathLibrary.MakeVector` _returnvalue_x_2 _returnvalue_y_2 _returnvalue_z)) false false)
  (if (not (`self.IsTalking`))
    (`self.ChooseRandomConversation`)
    (set `self.IsTalking` true))
  (`DialogueSystemComponent.DialogueInteract` (`self.DialogueSystemComponent`) null (`self.RandomConversationIndex`) true))

(event `self.InteractTrigger.OnComponentEndOverlap`
  (params (OverlappedComponent :type "PrimitiveComponent Object Reference") (OtherActor :type "Actor Object Reference") (OtherComp :type "PrimitiveComponent Object Reference") (OtherBodyIndex :type Integer))
  (if (`self.ActorHasTag` OtherActor "Player")
    (`DialogueSystemComponent.DisableDialogue` (`self.DialogueSystemComponent`) false)
    (`self.ReturnToWandering`)))

(event `self.DialogueSystemComponent.OnConversationEnd`
  (`self.ReturnToWandering`))

(event `ReturnToWandering`
  (`BlackboardComponent.SetValueAsBool` (`AIBlueprintHelperLibrary.GetBlackboard` null) (`KismetStringLibrary.Conv_StringToName` "bCanWander") true))

(fn `ChooseRandomConversation`
  (set `self.RandomConversationIndex` (`KismetMathLibrary.RandomIntegerInRange` 0 (- (`KismetArrayLibrary.Array_Length` (`DialogueSystemComponent.Conversations` (`self.DialogueSystemComponent`))) 1))))

(fn `UserConstructionScript`
  (`InteractableComponent.RegisterTriggerVolume` (`self.InteractableComponent`) (`self.InteractTrigger`)))