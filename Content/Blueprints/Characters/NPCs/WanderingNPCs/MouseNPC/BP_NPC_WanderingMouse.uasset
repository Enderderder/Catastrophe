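; Wandering mouse NPC that picks a random skin, roams under its AI controller and holds random conversations with the player.
; On interaction it halts via Blackboard flags, faces the player and runs dialogue, toggling the AnimBP talking state and resuming wandering when dialogue ends or the player leaves.
; The interact trigger shows a camera-facing speech bubble.
; Hits from BP_Tomato set a tripping flag in the Blackboard.
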(event `self.ReceiveBeginPlay`
  (bind _skins (`self.Skins`))
  ;[1 1 1] OnBeginPlay
  ;;[1 1 1] Randomly Choose skin
  (`PrimitiveComponent.SetMaterial` (`self.Mesh`) 0 (`|GetArrayItem` _skins (`KismetMathLibrary.RandomIntegerInRange` 0 (- (`KismetArrayLibrary.Array_Length` _skins) 1))))
  ;;[1 1 1] Initialise AI Variables
  (bind _asaic_npc_wandering_mouse (cast `/Game/Blueprints/Characters/NPCs/WanderingNPCs/MouseNPC/AIC_NPC_WanderingMouse` (`AIBlueprintHelperLibrary.GetAIController` self)))
  (`/Game/Blueprints/Characters/NPCs/WanderingNPCs/MouseNPC/AIC_NPC_WanderingMouse.Initialize` _asaic_npc_wandering_mouse (`self.bCanWander`) (`self.MinWanderDistance`) (`self.MaxWanderDistance`) (`self.MinWanderPauseTime`) (`self.MaxWanderPauseTime`) (`self.ChanceOfTripping`)))

(event `self.InteractableComponent.OnInteractSuccess`
  (params (_playerCharacter :type "PlayerCharacter Object Reference"))
  (bind _returnvalue (`AIBlueprintHelperLibrary.GetBlackboard` null))
  (bind (_returnvalue_x _returnvalue_y _returnvalue_z) (`KismetMathLibrary.BreakVector` (`self.K2_GetActorLocation`)))
  (bind (_returnvalue_x_2 _returnvalue_y_2) (`KismetMathLibrary.BreakVector` (`self.K2_GetActorLocation` _playerCharacter)))
  ;[1 1 1] On Interaction Use Dialogue
  (`MovementComponent.StopMovementImmediately` (`self.CharacterMovement`))
  (`BlackboardComponent.SetValueAsBool` _returnvalue (`KismetStringLibrary.Conv_StringToName` "bCanWander") false)
  (`BlackboardComponent.SetValueAsBool` _returnvalue (`KismetStringLibrary.Conv_StringToName` "bIsWandering") false)
  (`SceneComponent.K2_SetWorldRotation` (`self.CapsuleComponent`) (`KismetMathLibrary.FindLookAtRotation` (`self.K2_GetActorLocation`) (`KismetMathLibrary.MakeVector` _returnvalue_x_2 _returnvalue_y_2 _returnvalue_z)) false false)
  (if (not (`self.IsTalking`))
    (`self.ChooseRandomConversation`)
    (set `self.IsTalking` true))
  (`DialogueSystemComponent.DialogueInteract` (`self.DialogueSystemComponent`) null (`self.RandomConversationIndex`) true))

(event `self.InteractTrigger.OnComponentEndOverlap`
  (params (OverlappedComponent :type "PrimitiveComponent Object Reference") (OtherActor :type "Actor Object Reference") (OtherComp :type "PrimitiveComponent Object Reference") (OtherBodyIndex :type Integer))
  ;[1 1 1] Disable Dialogue If Walking Away
  (if (`self.ActorHasTag` OtherActor "Player")
    (`DialogueSystemComponent.DisableDialogue` (`self.DialogueSystemComponent`) false)
    (`self.ReturnToWandering`)
    (`SceneComponent.SetVisibility` (`self.SpeechBubble`) false false)))

(event `self.DialogueSystemComponent.OnConversationEnd`
  (params (ConversationIndex :type Integer))
  ;[1 1 1] On end of conversation
  (`self.ReturnToWandering`))

(event `ReturnToWandering`
  ;[1 1 1] Return to wander
  (`BlackboardComponent.SetValueAsBool` (`AIBlueprintHelperLibrary.GetBlackboard` null) (`KismetStringLibrary.Conv_StringToName` "bCanWander") true)
  (set `self.IsTalking` false))

(event `self.ReceiveTick`
  (params (DeltaSeconds :type "Float (single-precision)"))
  (bind _bubbleroot (`self.BubbleRoot`))
  (bind (_returnvalue_roll _returnvalue_pitch) (`KismetMathLibrary.BreakRotator` (`SceneComponent.K2_GetComponentRotation` _bubbleroot)))
  (bind (_returnvalue_roll_2 _returnvalue_pitch_2 _returnvalue_yaw) (`KismetMathLibrary.BreakRotator` (`KismetMathLibrary.FindLookAtRotation` (`SceneComponent.K2_GetComponentLocation` _bubbleroot) (`PlayerCameraManager.GetCameraLocation` (`GameplayStatics.GetPlayerCameraManager` 0)))))
  (if (`SceneComponent.IsVisible` (`self.SpeechBubble`))
    (`SceneComponent.K2_SetWorldRotation` (`self.BubbleRoot`) (`KismetMathLibrary.MakeRotator` _returnvalue_roll _returnvalue_pitch _returnvalue_yaw) false false)))

(event `self.InteractTrigger.OnComponentBeginOverlap`
  (params (OverlappedComponent :type "PrimitiveComponent Object Reference") (OtherActor :type "Actor Object Reference") (OtherComp :type "PrimitiveComponent Object Reference") (OtherBodyIndex :type Integer) (bFromSweep :type Boolean) (SweepResult :type "HitResult Structure (by ref)"))
  (if (`self.ActorHasTag` OtherActor "Player")
    (`SceneComponent.SetVisibility` (`self.SpeechBubble`) true false)))

(event `self.Mesh.OnComponentHit`
  (params (HitComponent :type "PrimitiveComponent Object Reference") (OtherActor :type "Actor Object Reference") (OtherComp :type "PrimitiveComponent Object Reference") (NormalImpulse :type "Vector Structure") (Hit :type "HitResult Structure (by ref)"))
  (cast `/Game/Blueprints/Items/BP_Tomato` OtherActor)
  (`BlackboardComponent.SetValueAsBool` (`AIBlueprintHelperLibrary.GetBlackboard` null) (`KismetStringLibrary.Conv_StringToName` "bIsTripping") true))

(event `self.DialogueSystemComponent.OnConversationStart`
  ;[1 1 1] Play talking animation
  (bind _asabp_mouse_npc (cast `/Game/Assets/MouseNPC/ABP_MouseNPC` (`SkeletalMeshComponent.GetAnimInstance` (`self.Mesh`))))
  (set `/Game/Assets/MouseNPC/ABP_MouseNPC.bTalking` true _asabp_mouse_npc))

(event `self.DialogueSystemComponent.OnDialogueDisable`
  ;[1 1 1] Stop talking animation
  (bind _asabp_mouse_npc (cast `/Game/Assets/MouseNPC/ABP_MouseNPC` (`SkeletalMeshComponent.GetAnimInstance` (`self.Mesh`))))
  (set `/Game/Assets/MouseNPC/ABP_MouseNPC.bTalking` false _asabp_mouse_npc))

(fn `ChooseRandomConversation`
  (set `self.RandomConversationIndex` (`KismetMathLibrary.RandomIntegerInRange` 0 (- (`KismetArrayLibrary.Array_Length` (`DialogueSystemComponent.Conversations` (`self.DialogueSystemComponent`))) 1))))

(fn `UserConstructionScript`
  (`InteractableComponent.RegisterTriggerVolume` (`self.InteractableComponent`) (`self.InteractTrigger`)))