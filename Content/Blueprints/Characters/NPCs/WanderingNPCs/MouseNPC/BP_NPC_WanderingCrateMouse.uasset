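; Wandering crate mouse NPC that picks a random skin from its Skins array on BeginPlay.
; It hands its wander distance, pause time and trip chance settings to AIC_NPC_WanderingMouse, which is initialized to run the AI.
; Hit events on the crate and body meshes are empty; disconnected leftover logic would set the bIsTripping blackboard key on BP_Tomato hits.
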(event `self.ReceiveBeginPlay`
  (bind _skins (`self.Skins`))
  ;[1 1 1] OnBeginPlay
  ;;[1 1 1] Randomly Choose skin
  (`PrimitiveComponent.SetMaterial` (`self.Mesh`) 0 (`|GetArrayItem` _skins (`KismetMathLibrary.RandomIntegerInRange` 0 (- (`KismetArrayLibrary.Array_Length` _skins) 1))))
  ;;[1 1 1] Initialise AI Variables
  (bind _asaic_npc_wandering_mouse (cast `/Game/Blueprints/Characters/NPCs/WanderingNPCs/MouseNPC/AIC_NPC_WanderingMouse` (`AIBlueprintHelperLibrary.GetAIController` self)))
  (`/Game/Blueprints/Characters/NPCs/WanderingNPCs/MouseNPC/AIC_NPC_WanderingMouse.Initialize` _asaic_npc_wandering_mouse (`self.bCanWander`) (`self.MinWanderDistance`) (`self.MaxWanderDistance`) (`self.MinWanderPauseTime`) (`self.MaxWanderPauseTime`) (`self.ChanceOfTripping`)))

(event `self.CrateMesh.OnComponentHit`
  (params (HitComponent :type "PrimitiveComponent Object Reference") (OtherActor :type "Actor Object Reference") (OtherComp :type "PrimitiveComponent Object Reference") (NormalImpulse :type "Vector Structure") (Hit :type "HitResult Structure (by ref)")))

(event `self.Mesh.OnComponentHit`
  (params (HitComponent :type "PrimitiveComponent Object Reference") (OtherActor :type "Actor Object Reference") (OtherComp :type "PrimitiveComponent Object Reference") (NormalImpulse :type "Vector Structure") (Hit :type "HitResult Structure (by ref)")))

(fn `UserConstructionScript`)