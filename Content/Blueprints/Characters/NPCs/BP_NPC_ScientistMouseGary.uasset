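; Gary the scientist mouse NPC, whose one-time conversation is tied to a Quest 3 objective and gates the hideout entrance.
; BeginPlay links the objective to the dialogue component and disables the entrance trigger's collision; interacting runs the conversation.
; Leaving the trigger box disables dialogue, and the disable event makes the player widget visible.
; Finishing the conversation hides the objective mesh, blocks further talking and re-enables the entrance trigger.
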(event `self.ReceiveBeginPlay`
  ;[1 1 1] Linking Quests with Dialogue System
  (bind _asbp_player_character (cast `/Game/Blueprints/Characters/Player/BP_PlayerCharacter` (`GameplayStatics.GetPlayerCharacter` 0)))
  (set `self.Player` _asbp_player_character)
  (`DialogueSystemComponent.AttachQuestObjectiveToConversation` (`self.DialogueSystemComponent`) 0 (`self.Quest3Objective0`))
  (`PrimitiveComponent.SetCollisionEnabled` (`/Game/Blueprints/ScuffShit/BP_Teleporter.Trigger` (`self.HideoutEntrance`)) "NoCollision"))

(event `self.TriggerBox.OnComponentEndOverlap`
  (params (OverlappedComponent :type "PrimitiveComponent Object Reference") (OtherActor :type "Actor Object Reference") (OtherComp :type "PrimitiveComponent Object Reference") (OtherBodyIndex :type Integer))
  ;[1 1 1] Stops Dialogue When Player Walks Away
  (cast `/Game/Blueprints/Characters/Player/BP_PlayerCharacter` OtherActor)
  (`DialogueSystemComponent.DisableDialogue` (`self.DialogueSystemComponent`) false))

(event `self.Receive_Interact`
  ;[1 1 1] OnInteract
  (`DialogueSystemComponent.DialogueInteract` (`self.DialogueSystemComponent`) (`self.Player`) 0 (`self.CanTalk`)))

(event `self.DialogueSystemComponent.OnDialogueDisable`
  (`Widget.SetVisibility` (`PlayerCharacter.PlayerWidget` (`self.Player`)) "Visible"))

(event `self.DialogueSystemComponent.OnConversationEnd`
  (`SceneComponent.SetVisibility` (`self.ObjectiveMesh`) false false)
  (set `self.CanTalk` false)
  (`PrimitiveComponent.SetCollisionEnabled` (`/Game/Blueprints/ScuffShit/BP_Teleporter.Trigger` (`self.HideoutEntrance`)) "QueryAndPhysics"))

(fn `UserConstructionScript`)