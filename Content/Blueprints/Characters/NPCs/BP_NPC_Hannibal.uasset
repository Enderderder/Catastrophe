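; BP_NPC_Hannibal is an NPC the player can interact with to hold a randomly chosen conversation.
; On interaction it picks a random conversation index if not already talking, then passes it to DialogueSystemComponent, so repeat interactions stay in the same conversation.
; Conversation end clears the Talking flag, and a player-tagged actor leaving the TriggerBox disables the dialogue.
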(event `self.InteractableComponent.OnInteractSuccess`
  (params (_playerCharacter :type "PlayerCharacter Object Reference"))
  (if (not (`self.bTalking`))
    (`self.ChooseRandomConversation`)
    (set `self.bTalking` true))
  (`DialogueSystemComponent.DialogueInteract` (`self.DialogueSystemComponent`) _playerCharacter (`self.RandomConversationIndex`) true))

(event `self.DialogueSystemComponent.OnConversationEnd`
  (params (ConversationIndex :type Integer))
  (set `self.bTalking` false))

(event `self.TriggerBox.OnComponentEndOverlap`
  (params (OverlappedComponent :type "PrimitiveComponent Object Reference") (OtherActor :type "Actor Object Reference") (OtherComp :type "PrimitiveComponent Object Reference") (OtherBodyIndex :type Integer))
  (if (`self.ActorHasTag` OtherActor "Player")
    (`DialogueSystemComponent.DisableDialogue` (`self.DialogueSystemComponent`) false)))

(fn `ChooseRandomConversation`
  (set `self.RandomConversationIndex` (`KismetMathLibrary.RandomIntegerInRange` 0 (- (`KismetArrayLibrary.Array_Length` (`DialogueSystemComponent.Conversations` (`self.DialogueSystemComponent`))) 1))))

(fn `UserConstructionScript`)