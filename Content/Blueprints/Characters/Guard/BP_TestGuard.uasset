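; Test guard character that shows sleep, question and alert indicators and sends a caught player to the HoldingCell.
; Indicator toggles drive mesh AnimBPs, clearing the others when enabled, and the catch hitbox loads and respawns through the respawn subsystem.
; State changes run old/new switches, where only wake-up stage one acts, using a timer to return to sleep.
; A makeshift hearing sphere tracks player proximity, but its movement-based wake-up logic is disconnected.
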(event `self.ToggleZzzIndicator`
  (params (_b :type Boolean))
  ;[1 1 1] Indicator toggles
  (bind _zzzaniminstance (`self.GetZzzAnimInstance`)
    (:`Output`
      (bind _output_get (set `/Game/Assets/Zzz/ABP_Zzz.bOn` _b _zzzaniminstance))
      (if _output_get
        (bind _abp_alert (`self.GetAlertAnimInstance`)
          (:`Success`
            (set `/Game/Assets/Alert/ABP_Alert.bAlerted` false _abp_alert)
            (bind _abp_questionmark (`self.GetQuestionMarkAnimInstance`)
              (:`Success`
                (set `/Game/Assets/Questionmark/ABP_QuestionMark.bQuestioning` false _abp_questionmark)))))))))

(event `self.ToggleQuestionIndicator`
  (params (_b :type Boolean))
  ;[1 1 1] Indicator toggles
  (bind _abp_questionmark (`self.GetQuestionMarkAnimInstance`)
    (:`Success`
      (bind _output_get (set `/Game/Assets/Questionmark/ABP_QuestionMark.bQuestioning` _b _abp_questionmark))
      (if _output_get
        (bind _abp_alert (`self.GetAlertAnimInstance`)
          (:`Success`
            (set `/Game/Assets/Alert/ABP_Alert.bAlerted` false _abp_alert)
            (bind _zzzaniminstance (`self.GetZzzAnimInstance`)
              (:`Output`
                (set `/Game/Assets/Zzz/ABP_Zzz.bOn` false _zzzaniminstance)))))))))

(event `self.ToggleAlertIndicator`
  (params (_b :type Boolean))
  ;[1 1 1] Indicator toggles
  (bind _abp_alert (`self.GetAlertAnimInstance`)
    (:`Success`
      (bind _output_get (set `/Game/Assets/Alert/ABP_Alert.bAlerted` _b _abp_alert))
      (if _output_get
        (bind _abp_questionmark (`self.GetQuestionMarkAnimInstance`)
          (:`Success`
            (set `/Game/Assets/Questionmark/ABP_QuestionMark.bQuestioning` false _abp_questionmark)
            (bind _zzzaniminstance (`self.GetZzzAnimInstance`)
              (:`Output`
                (set `/Game/Assets/Zzz/ABP_Zzz.bOn` false _zzzaniminstance)))))))))

(event `self.CatchHitBox.OnComponentBeginOverlap`
  (params (OverlappedComponent :type "PrimitiveComponent Object Reference") (OtherActor :type "Actor Object Reference") (OtherComp :type "PrimitiveComponent Object Reference") (OtherBodyIndex :type Integer) (bFromSweep :type Boolean) (SweepResult :type "HitResult Structure (by ref)"))
  (bind _returnvalue (subsystem `RespawnSubsystem`))
  ;[1 1 1] Catch player
  (if (`self.ActorHasTag` OtherActor "Player")
    (bind _returnvalue_2 (`RespawnSubsystem.GetStreamingLevelNameFromActor` _returnvalue self))
    (`RespawnSubsystem.LoadLevelStreaming` _returnvalue (make `LoadStreamingLevelInfo` _returnvalue_2 "HoldingCell" true true "HOLDINGCELL"))
    (`RespawnSubsystem.RespawnPlayerAtLocation` _returnvalue "HOLDINGCELL")))

(event `self.Receive_OnStunBegin`
  ;[1 1 1] Stun VFX
  (`GameplayStatics.SpawnEmitterAtLocation` "/Game/VFX/Stun/P_Stun.P_Stun" (`SceneComponent.K2_GetComponentLocation` (`self.StunVfxLocation`))))

(event `self.ReceiveTick`
  (params (DeltaSeconds :type "Float (single-precision)"))
  ;[1 1 1] Testing Shit
  (switch `EGuardState` (`self.GuardState`)))

(event `ReturnToSleep`
  ;[1 1 1] When the state of guard changes
  (`self.SetGuardState` "SLEEPING"))

(event `self.OnGuardStateChange`
  (params (_oldState :type "EGuardState Enum" :default "STATIONARY") (_newState :type "EGuardState Enum" :default "STATIONARY"))
  ;[1 1 1] When the state of guard changes
  (`parent.OnGuardStateChange` _oldState _newState)
  (switch `EGuardState` _oldState
    (:`STATIONARY`
      _)
    (:`SLEEPING`
      _)
    (:`WAKEUP_STAGEONE`
      (`KismetSystemLibrary.K2_ClearAndInvalidateTimerHandle` (`self.WakeUpStageOneTimerHandle_0`)))
    (:`WAKEUP_STAGETWO`
      _)
    (:`PATROLLING`
      _)
    (:`INVESTATING`
      _)
    (:`CHASING`
      _)
    (:`SEARCHING`
      _)
    (:`STUNED`
      _))
  (switch `EGuardState` _newState
    (:`STATIONARY`)
    (:`SLEEPING`)
    (:`WAKEUP_STAGEONE`
      (bind _returnvalue (`KismetSystemLibrary.K2_SetTimerDelegate` (delegate `ReturnToSleep`) 3.0))
      (set `self.WakeUpStageOneTimerHandle_0` _returnvalue))
    (:`WAKEUP_STAGETWO`)
    (:`PATROLLING`)
    (:`INVESTATING`)
    (:`CHASING`)
    (:`SEARCHING`)
    (:`STUNED`)))

(event `self.StupidFakeBsHearingSphere.OnComponentBeginOverlap`
  (params (OverlappedComponent :type "PrimitiveComponent Object Reference") (OtherActor :type "Actor Object Reference") (OtherComp :type "PrimitiveComponent Object Reference") (OtherBodyIndex :type Integer) (bFromSweep :type Boolean) (SweepResult :type "HitResult Structure (by ref)"))
  ;[1 1 1] Stupid hearing sphere detection
  (if (`self.ActorHasTag` OtherActor "Player")
    (set `self.bPlayerInSleepDetectRange` true)))

(event `self.StupidFakeBsHearingSphere.OnComponentEndOverlap`
  (params (OverlappedComponent :type "PrimitiveComponent Object Reference") (OtherActor :type "Actor Object Reference") (OtherComp :type "PrimitiveComponent Object Reference") (OtherBodyIndex :type Integer))
  ;[1 1 1] Stupid hearing sphere detection
  (if (`self.ActorHasTag` OtherActor "Player")
    (set `self.bPlayerInSleepDetectRange` false)))

(fn `GetPerceptionLocRot`
  (returns (Location :type "Vector Structure") (Rotation :type "Rotator Structure"))
  (bind (_returnvalue_location _returnvalue_rotation) (`KismetMathLibrary.BreakTransform` (`SceneComponent.GetSocketTransform` (`self.Mesh`) "PerceptionSocket" "RTS_World")))
  (return _returnvalue_location _returnvalue_rotation))

(fn `LookAround`
  (returns (out_montageTime :type "Float (double-precision)"))
  (bind _guardaniminstance (`self.GuardAnimInstance`)
    (:`then`
      (bind _returnvalue (`AnimInstance.Montage_Play` _guardaniminstance "/Game/Assets/Guard/Animations/AM_Guard_Search_LookUp.AM_Guard_Search_LookUp" 1.0 "Duration" 0.0 true))
      (return _returnvalue))
    (:`else`
      (return 0.0))))

(fn `UserConstructionScript`)