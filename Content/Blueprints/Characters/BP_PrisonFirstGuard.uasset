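; BP_PrisonFirstGuard is a guard character that serves as the target for the third objective of Quest 0.
; Its objective marker starts hidden, and Tick polls the objective state each frame to show the marker while that objective is active.
; When a stun begins on the guard, it completes the objective and hides the marker.
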(event `self.ReceiveBeginPlay`
  (`SceneComponent.SetVisibility` (`self.ObjectiveMarker`) false false))

(event `self.ReceiveTick`
  (params (DeltaSeconds :type "Float (single-precision)"))
  (`parent.ReceiveTick` DeltaSeconds)
  (if (`|EnumEquality` (`QuestObjectiveComponent.ObjectiveState` (`self.Quest0Objective3`)) "Active")
    (`SceneComponent.SetVisibility` (`self.ObjectiveMarker`) true false)))

(event `self.Receive_OnStunBegin`
  (`QuestObjectiveComponent.CompleteObjective` (`self.Quest0Objective3`))
  (`SceneComponent.SetVisibility` (`self.ObjectiveMarker`) false false))

(fn `UserConstructionScript`
  (`parent.UserConstructionScript`))