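; Catnip ball pickup that acts as the game-ending interactable.
; On successful interaction it destroys its mesh, has the game mode play the end cutscene and hides the player after short delays.
; When the cutscene finishes it spawns BP_Prologue and unhides the player.
; When the prologue finishes, the respawn subsystem returns the player to the HUB district at the "From Market" location.
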(event `self.InteractableComponent.OnInteractSuccess`
  (params (_playerCharacter :type "PlayerCharacter Object Reference"))
  ;[0.1 0.1 0.1] Play cutscene, game end
  (`KismetSystemLibrary.Delay` 0.2)
  (`ActorComponent.K2_DestroyComponent` (`self.ItemMesh`))
  (bind _return_value (`/Game/Blueprints/Gameplay/Gamemodes/BP_CatastropheMainGameMode.PlayCutscene` :`self` (cast `/Game/Blueprints/Gameplay/Gamemodes/BP_CatastropheMainGameMode` (`GameplayStatics.GetGameMode`) :!pure true) :`Cutscene` "/Game/Sequences/S_End.S_End"))
  (add `MovieSceneSequencePlayer.OnFinished` _return_value (delegate `OnFinished`))
  (`KismetSystemLibrary.Delay` 1.0)
  (`self.SetActorHiddenInGame` _playerCharacter true))

(event `OnFinished`
  ;[0.1 0.1 0.1] Play cutscene, game end
  (bind _returnvalue (`|SpawnActorFromClass` "/Game/Blueprints/Gameplay/BP_Prologue.BP_Prologue_C" (`KismetMathLibrary.MakeTransform` (0.0 0.0 0.0)) "Undefined" "OverrideRootScale" null null))
  (add `/Game/Blueprints/Gameplay/BP_Prologue.OnPrologueFinish` _returnvalue (delegate `OnPrologueFinish`))
  (`self.SetActorHiddenInGame` (stale `self.InteractableComponent.OnInteractSuccess` _playerCharacter) false))

(event `OnPrologueFinish`
  ;[0.1 0.1 0.1] Play cutscene, game end
  (`RespawnSubsystem.RespawnPlayerAtDistrict` (subsystem `RespawnSubsystem`) "HUB" "From Market"))

(fn `UserConstructionScript`
  (`parent.UserConstructionScript`))