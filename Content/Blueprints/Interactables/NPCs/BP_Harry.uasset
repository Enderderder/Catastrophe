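; BP_Harry is a quest-giver NPC with a dialogue widget and quest objectives.
; BeginPlay caches the player and links quests to the first conversation; leaving the trigger box ends dialogue.
; Widget updates set both speakers' lines and show the active speaker's icon.
; Finishing the old or new quest adds fishbones to the player, while two objective components print activation and completion messages with the task text left empty.
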(event `self.ReceiveBeginPlay`
  ;[1 1 1] Linking Quests components with dialogue system
  (bind _asbp_player_character (cast `/Game/Blueprints/Characters/BP_PlayerCharacter` (`GameplayStatics.GetPlayerCharacter` 0)))
  (set `self.Player` _asbp_player_character)
  (for (_ _array_index) (`self.ConversationsList`)
    (switch `int` _array_index
      (:`0`
        (`self.SetConversationQuests` _array_index)))))

(event `self.Receive_UpdateWidget`
  (bind _dialoguewidget (`self.DialogueWidget`))
  ;[1 1 1] Updating Dialogue Widget
  (bind _aswbp_dialogue (cast `/Game/Assets/UI/Widgets/Dialogue/WBP_Dialogue` (`self.DialogueWidget`)))
  (`TextBlock.SetText` (`/Game/Assets/UI/Widgets/Dialogue/WBP_Dialogue.NPC_Text` _aswbp_dialogue) (`KismetTextLibrary.Conv_StringToText` (`self.CurrentNPCDialogueText`)))
  (`TextBlock.SetText` (`/Game/Assets/UI/Widgets/Dialogue/WBP_Dialogue.Player_Text` _aswbp_dialogue) (`KismetTextLibrary.Conv_StringToText` (`self.CurrentPlayerDialogueText`)))
  (bind _aswbp_dialogue_2 (cast `/Game/Assets/UI/Widgets/Dialogue/WBP_Dialogue` (`self.DialogueWidget`)))
  (bind _npc_icon (`/Game/Assets/UI/Widgets/Dialogue/WBP_Dialogue.NPC_Icon` _aswbp_dialogue_2))
  (`Image.SetBrush` _npc_icon (make `SlateBrush` (`Widget.GetDesiredSize` _npc_icon) (struct) (struct :`SpecifiedColor` (struct :`R` 1.0 :`G` 1.0 :`B` 1.0 :`A` 1.0) :`ColorUseRule` "UseColor_Specified") (`self.NPCIcon`)))
  (if (`self.IsNPCTalking`)
    (bind _aswbp_dialogue_3 (cast `/Game/Assets/UI/Widgets/Dialogue/WBP_Dialogue` _dialoguewidget))
    (`Widget.SetVisibility` (`/Game/Assets/UI/Widgets/Dialogue/WBP_Dialogue.NPC_Icon` _aswbp_dialogue_3) "Visible")
    (`Widget.SetVisibility` (`/Game/Assets/UI/Widgets/Dialogue/WBP_Dialogue.Player_Icon` _aswbp_dialogue_3) "Hidden")
    (else
      (bind _aswbp_dialogue_4 (cast `/Game/Assets/UI/Widgets/Dialogue/WBP_Dialogue` _dialoguewidget))
      (`Widget.SetVisibility` (`/Game/Assets/UI/Widgets/Dialogue/WBP_Dialogue.NPC_Icon` _aswbp_dialogue_4) "Hidden")
      (`Widget.SetVisibility` (`/Game/Assets/UI/Widgets/Dialogue/WBP_Dialogue.Player_Icon` _aswbp_dialogue_4) "Visible"))))

(event `self.TriggerBox.OnComponentEndOverlap`
  (params (OverlappedComponent :type "PrimitiveComponent Object Reference") (OtherActor :type "Actor Object Reference") (OtherComp :type "PrimitiveComponent Object Reference") (OtherBodyIndex :type Integer))
  ;[1 1 1] Stops dialogue when player walks away
  (cast `/Game/Blueprints/Characters/BP_PlayerCharacter` OtherActor)
  (`self.DisableDialogue`))

(event `self.Receive_FinishOldQuest`
  ;[1 1 1] OnFinish of OldQuest
  (bind _returnvalue (`self.GetCurrentFishboneReward_OldQuest`))
  (set `PlayerCharacter.FishBonesAmount` (+ _returnvalue (`PlayerCharacter.FishBonesAmount` (`self.Player`))) (`self.Player`)))

(event `self.Receive_FinishNewQuest`
  ;[1 1 1] OnFinish of NewQuest
  (bind _returnvalue (`self.GetCurrentFishboneReward_NewQuest`))
  (set `PlayerCharacter.FishBonesAmount` (+ _returnvalue (`PlayerCharacter.FishBonesAmount` (`self.Player`))) (`self.Player`)))

(event `self.QuestObjective1.OnObjectiveActivate`
  ;[1 1 1] Printing to screen when Quests activated/completed
  (`KismetSystemLibrary.PrintString` (`KismetStringLibrary.Concat_StrStr` "New Task: ") true true (struct :`G` 0.66 :`B` 1.0 :`A` 1.0) 5.0))

(event `self.QuestObjective1.OnObjectiveComplete`
  ;[1 1 1] Printing to screen when Quests activated/completed
  (`KismetSystemLibrary.PrintString` (`KismetStringLibrary.Concat_StrStr` "Task Completed: ") true true (struct :`G` 0.53125 :`B` 0.067013 :`A` 1.0) 5.0))

(event `self.QuestObjective2.OnObjectiveActivate`
  ;[1 1 1] Printing to screen when Quests activated/completed
  (`KismetSystemLibrary.PrintString` (`KismetStringLibrary.Concat_StrStr` "New Task: ") true true (struct :`G` 0.66 :`B` 1.0 :`A` 1.0) 5.0))

(event `self.QuestObjective2.OnObjectiveComplete`
  ;[1 1 1] Printing to screen when Quests activated/completed
  (`KismetSystemLibrary.PrintString` (`KismetStringLibrary.Concat_StrStr` "Task Completed: ") true true (struct :`G` 0.533276 :`B` 0.066626 :`A` 1.0) 5.0))

(fn `UserConstructionScript`)