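; BP_Shop is a shop interactable, filed under NPCs, that hands control between gameplay and a shop UI.
; On BeginPlay it calls WidgetInit with WBP_Shop.
; Enabling the shop gives the widget a reference back to this actor, shows the cursor, disables player movement and switches to UI-only input.
; Disabling it restores game-only input, hides the cursor and sets movement back to walking.
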(event `self.ReceiveBeginPlay`
  (`self.WidgetInit` "/Game/Assets/UI/Widgets/WBP_Shop.WBP_Shop_C"))

(event `self.Receive_EnableShop`
  (bind _returnvalue (`GameplayStatics.GetPlayerController` 0))
  (bind _aswbp_shop (cast `/Game/Assets/UI/Widgets/WBP_Shop` (`self.ShopWidget`)))
  (set `/Game/Assets/UI/Widgets/WBP_Shop.Shop` self _aswbp_shop)
  (set `PlayerController.bShowMouseCursor` true _returnvalue)
  (`CharacterMovementComponent.DisableMovement` (`Character.CharacterMovement` (`GameplayStatics.GetPlayerCharacter` 0)))
  (`WidgetBlueprintLibrary.SetInputMode_UIOnlyEx` _returnvalue null))

(event `self.Receive_DisableShop`
  (bind _returnvalue (`GameplayStatics.GetPlayerController` 0))
  (`WidgetBlueprintLibrary.SetInputMode_GameOnly` _returnvalue)
  (set `PlayerController.bShowMouseCursor` false _returnvalue)
  (`CharacterMovementComponent.SetMovementMode` (`Character.CharacterMovement` (`GameplayStatics.GetPlayerCharacter` 0)) "MOVE_Walking" 0))

(fn `UserConstructionScript`)