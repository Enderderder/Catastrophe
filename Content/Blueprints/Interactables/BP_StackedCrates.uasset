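; BP_StackedCrates is an interactable stack of crates that can fall and become a blocking obstacle.
; BeginPlay caches the mesh's ABP_FallingCrate anim instance and disables collision on BlockVolume.
; The _PlayCrateAnim event sets the Fallen flag to drive the animation, then enables BlockVolume collision after a short delay.
; Interacting only turns off the mesh's custom depth rendering; nothing in this graph calls the fall event.
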(event `self.InteractableComponent.OnInteract`
  (params (_playerCharacter :type "PlayerCharacter Object Reference"))
  (`PrimitiveComponent.SetRenderCustomDepth` (`self.CratesMesh`) false))

(event `self.ReceiveBeginPlay`
  ;[1 1 1] Begin Play
  (set `self.AnimInstance` (cast `/Game/Assets/Kitsets/Kitset_Market/FallingCrates/ABP_FallingCrate` (`SkeletalMeshComponent.GetAnimInstance` (`self.CratesMesh`)) :!pure true))
  (`PrimitiveComponent.SetCollisionEnabled` (`self.BlockVolume`) "NoCollision"))

(event `self.Receive_PlayCrateAnim`
  ;[1 1 1] Crate Fallen Anim
  (set `/Game/Assets/Kitsets/Kitset_Market/FallingCrates/ABP_FallingCrate.bFallen` true (`self.AnimInstance`))
  (`KismetSystemLibrary.Delay` 0.4)
  (`PrimitiveComponent.SetCollisionEnabled` (`self.BlockVolume`) "QueryAndPhysics"))

(fn `UserConstructionScript`
  (`parent.UserConstructionScript`))