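; BP_JailUrn is an interactable jail urn tied to a quest objective that the player can jump into.
; Tick enables interaction and shows the objective marker only while its QuestObjective is active.
; Jumping in plays the S_GuardOpeningCell level sequence and completes the objective.
; BeginPlay caches the player's quest widget, which this graph does not otherwise use.
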(event `self.ReceiveBeginPlay`
  (`parent.ReceiveBeginPlay`)
  ;[1 1 1] Get Quest Widget
  (bind _asbp_player_character (cast `/Game/Blueprints/Characters/BP_PlayerCharacter` (`GameplayStatics.GetPlayerCharacter` 0)))
  (set `self.QuestWidget` (`/Game/Blueprints/Characters/BP_PlayerCharacter.QuestWidget` _asbp_player_character)))

(event `self.ReceiveTick`
  (params (DeltaSeconds :type "Float (single-precision)"))
  (bind _output_get (set `self.bCanInteract` (`QuestObjectiveComponent.IsObjectiveActive` (`self.QuestObjective`))))
  (if _output_get
    (`SceneComponent.SetVisibility` (`self.ObjectiveMarker`) true false)
    (else
      (`SceneComponent.SetVisibility` (`self.ObjectiveMarker`) false false))))

(event `self.Receive_JumpIn`
  (params (_playerCharacter :type "PlayerCharacter Object Reference"))
  (bind (_outactor _returnvalue) (`LevelSequencePlayer.CreateLevelSequencePlayer` "/Game/Sequences/S_GuardOpeningCell.S_GuardOpeningCell"))
  (`MovieSceneSequencePlayer.Play` _returnvalue)
  (`QuestObjectiveComponent.CompleteObjective` (`self.QuestObjective`)))

(event `self.QuestObjective.OnObjectiveActivate`
  ;[1 1 1] Print to screen when Quests activated/completed
)

(event `self.QuestObjective.OnObjectiveComplete`
  ;[1 1 1] Print to screen when Quests activated/completed
)

(fn `UserConstructionScript`
  (`parent.UserConstructionScript`))