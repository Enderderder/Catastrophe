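; BP_Catnip is an interactable catnip pickup that boosts the movement of the player who uses it.
; The construction script registers its Box as the Interactable trigger volume.
; A successful interaction applies a timed speed modifier through the player's MovementModifierComponent and sets a fixed jump velocity, which this Blueprint never restores.
; A disconnected chain that would remove the pickup and temporarily enable a Trip effect never runs.
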(event `self.Interactable.OnInteractSuccess`
  (params (_playerCharacter :type "PlayerCharacter Object Reference"))
  (`MovementModifierComponent.ApplySpeedModifierWithDurationToAll` (`PlayerCharacter.MovementModifierComponent` _playerCharacter) (`self.SpeedModifierIncrease`) (`self.EffectDuration`))
  (set `CharacterMovementComponent.JumpZVelocity` 1500.0 (`Character.CharacterMovement` _playerCharacter)))

(fn `UserConstructionScript`
  (`parent.UserConstructionScript`)
  (`InteractableComponent.RegisterTriggerVolume` (`self.Interactable`) (`self.Box`)))