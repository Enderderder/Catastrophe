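; BP_HideoutJailDoor is a jail door whose gate opens when a BP_Tomato hits its TomatoTrigger component.
; The hit destroys the tomato and, if DoorOpen is false, plays a timeline that offsets the gate from the start location cached at BeginPlay.
; DoorOpen is never set here, so later hits replay the opening from the start.
; A second timeline for closing exists but is not connected.
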(event `self.TomatoTrigger.OnComponentHit`
  (params (HitComponent :type "PrimitiveComponent Object Reference") (OtherActor :type "Actor Object Reference") (OtherComp :type "PrimitiveComponent Object Reference") (NormalImpulse :type "Vector Structure") (Hit :type "HitResult Structure (by ref)"))
  (bind _asbp_tomato (cast `/Game/Blueprints/Items/BP_Tomato` OtherActor))
  (`self.K2_DestroyActor` _asbp_tomato)
  (if (not (`self.Door_Open`))
    ;[1 1 1] open door
    (bind (_direction _newtrack_0) (`Timeline|Timeline_0` :!via `PlayFromStart`)
      (:`Update`
        (bind _returnvalue (- (`self.Door_Start`) _newtrack_0))
        (set `self.Door_End` _returnvalue)
        (`SceneComponent.K2_SetWorldLocation` (`self.gate`) _returnvalue false false)))))

(event `self.ReceiveBeginPlay`
  (set `self.Door_Start` (`SceneComponent.K2_GetComponentLocation` (`self.gate`))))

(fn `UserConstructionScript`)