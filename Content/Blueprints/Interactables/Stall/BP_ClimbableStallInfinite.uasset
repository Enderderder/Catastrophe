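; BP_ClimbableStallInfinite is an interactable market stall variant for climbing, built on a parent class.
; On begin play it fills the waypoint array with three waypoints that define the climb path.
; Interacting turns off the mesh's custom depth rendering.
; When the interaction ends, it destroys the climb mesh and reveals a ripped carpet.
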(event `self.ReceiveBeginPlay`
  (bind _waypointarray (`self.WayPointArray`))
  ;[1 1 1] Setup the array of way point  for climbing
  (`KismetArrayLibrary.Array_Clear` _waypointarray)
  (`KismetArrayLibrary.Array_Append` _waypointarray (`|MakeArray` (`self.WayPoint_1`) (`self.WayPoint_2`) (`self.WayPoint_3`))))

(event `self.Recieve_InteractionEnd`
  ;[1 1 1] OnUse
  (`ActorComponent.K2_DestroyComponent` (`self.ClimbMesh`))
  (`SceneComponent.SetVisibility` (`self.RippedCarpet`) true false))

(event `self.InteractableComponent.OnInteract`
  (params (_playerCharacter :type "PlayerCharacter Object Reference"))
  (`PrimitiveComponent.SetRenderCustomDepth` (`self.Mesh`) false))

(fn `UserConstructionScript`
  (`parent.UserConstructionScript`))