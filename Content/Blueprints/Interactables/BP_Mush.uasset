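; BP_Mush is an interactable mushroom pickup that switches on a timed "Trip" effect when used.
; The construction script registers its Box with the Interactable component as the trigger volume.
; On interact, it removes the Box and mushroom, prints a debug greeting, and enables Trip.
; The actor stays alive through a one-minute delay, then disables Trip and destroys itself.
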(event `self.Interactable.OnInteract`
  (params (_playerCharacter :type "PlayerCharacter Object Reference"))
  (`ActorComponent.K2_DestroyComponent` (`self.Box`))
  (`ActorComponent.K2_DestroyComponent` (`self.Mush`))
  (`KismetSystemLibrary.PrintString` "Hello")
  (set `PostProcessComponent.bEnabled` true (`self.Trip`))
  (`KismetSystemLibrary.Delay` 60.0)
  (set `PostProcessComponent.bEnabled` false (`self.Trip`))
  (`self.K2_DestroyActor`))

(fn `UserConstructionScript`
  (`parent.UserConstructionScript`)
  (`InteractableComponent.RegisterTriggerVolume` (`self.Interactable`) (`self.Box`)))