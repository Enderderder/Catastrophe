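; BP_TutorialStackedCrates is an interactable crate stack that serves as a tutorial quest objective.
; Tick shows the ObjectiveMarker only while its QuestObjective is Active, polling the state every frame.
; Player interaction calls CompleteObjective on the QuestObjective without checking its state in this graph.
; The objective's activate and complete events print the task's short description to the screen.
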(event `self.ReceiveTick`
  (params (DeltaSeconds :type "Float (single-precision)"))
  (bind _objectivemarker (`self.ObjectiveMarker`))
  (if (`|EnumEquality` (`QuestObjectiveComponent.ObjectiveState` (`self.QuestObjective`)) "Active")
    (`SceneComponent.SetVisibility` _objectivemarker true false)
    (else
      (`SceneComponent.SetVisibility` _objectivemarker false false))))

(event `self.Receive_OnPlayerInteract`
  ;[1 1 1] Complete Objective when interact
  (`QuestObjectiveComponent.CompleteObjective` (`self.QuestObjective`)))

(event `self.QuestObjective.OnObjectiveActivate`
  ;[1 1 1] Print to screen when QuestObjective is activated/completed
  (`KismetSystemLibrary.PrintString` (`KismetStringLibrary.Concat_StrStr` "New Task: " (`QuestObjectiveComponent.ShortDescription` (`self.QuestObjective`)))))

(event `self.QuestObjective.OnObjectiveComplete`
  ;[1 1 1] Print to screen when QuestObjective is activated/completed
  (`KismetSystemLibrary.PrintString` (`KismetStringLibrary.Concat_StrStr` "Task Completed: " (`QuestObjectiveComponent.ShortDescription` (`self.QuestObjective`)))))

(fn `UserConstructionScript`
  (`parent.UserConstructionScript`))