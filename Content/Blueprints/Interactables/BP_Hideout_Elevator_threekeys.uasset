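; Hideout elevator interactable that opens only after three keys, which are components of the same actor, have been picked up.
; Each key's interactable, bound to its own trigger volume in the construction script, sets a flag and destroys that key's mesh and collision.
; With all three flags set, the main interactable plays a timeline that offsets ElevatorBody from its starting location.
; An older open/close door toggle remains but never runs.
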(event `self.ReceiveBeginPlay`
  (set `self.Door_Start` (`SceneComponent.K2_GetComponentLocation` (`self.elevator_Body`))))

(event `self.Interactable.OnInteractSuccess`
  (params (_playerCharacter :type "PlayerCharacter Object Reference"))
  (if (and (`self.Key_1`) (`self.Key_2`) (`self.Key_3`))
    ;[1 1 1] open gates
    (bind (_direction _newtrack_0) (`Timeline|Door_close`)
      (:`Update`
        (`SceneComponent.K2_SetWorldLocation` (`self.elevator_Body`) (+ (`self.Door_Start`) _newtrack_0) false false)))))

(event `self.InteractableKey1.OnInteractSuccess`
  (params (_playerCharacter :type "PlayerCharacter Object Reference"))
  (set `self.Key_1` true)
  (`ActorComponent.K2_DestroyComponent` (`self.key`))
  (`ActorComponent.K2_DestroyComponent` (`self.key_collision1`)))

(event `self.InteractableKey2.OnInteractSuccess`
  (params (_playerCharacter :type "PlayerCharacter Object Reference"))
  (set `self.Key_2` true)
  (`ActorComponent.K2_DestroyComponent` (`self.key2`))
  (`ActorComponent.K2_DestroyComponent` (`self.key_collision2`)))

(event `self.InteractableKey3.OnInteractSuccess`
  (params (_playerCharacter :type "PlayerCharacter Object Reference"))
  (set `self.Key_3` true)
  (`ActorComponent.K2_DestroyComponent` (`self.key3`))
  (`ActorComponent.K2_DestroyComponent` (`self.key_collision3`)))

(fn `UserConstructionScript`
  (`InteractableComponent.RegisterTriggerVolume` (`self.Interactable`) (`self.Box`))
  (`InteractableComponent.RegisterTriggerVolume` (`self.InteractableKey1`) (`self.key_collision1`))
  (`InteractableComponent.RegisterTriggerVolume` (`self.InteractableKey2`) (`self.key_collision2`))
  (`InteractableComponent.RegisterTriggerVolume` (`self.InteractableKey3`) (`self.key_collision3`)))