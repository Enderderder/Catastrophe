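; Hideout door actor that players toggle open and closed through its Interactable component.
; The construction script registers the Box as the trigger volume, and BeginPlay caches the Cube's starting world location.
; Separate open and close timelines slide the Cube by world-space offsets, with closing based on the last position recorded while opening.
; Timeline updates also set the open flag and switch the interaction prompt.
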(event `self.ReceiveBeginPlay`
  (set `self.Door_Start` (`SceneComponent.K2_GetComponentLocation` (`self.Cube`))))

(event `self.Interactable.OnInteractSuccess`
  (params (_playerCharacter :type "PlayerCharacter Object Reference"))
  (bind _cube (`self.Cube`))
  (if (`self.Door_Open`)
    ;[1 1 1] close door
    (bind (_direction _newtrack_0) (`Timeline|Door_close` :!via `PlayFromStart`)
      (:`Update`
        (`SceneComponent.K2_SetWorldLocation` _cube (+ (`self.Door_End`) _newtrack_0) false false)
        (set `self.Door_Open` false)
        (set `InteractableComponent.InteractionDescriptionText` "Open Door" (`self.Interactable`))))
    (else
      ;[1 1 1] open door
      (bind (_direction_2 _newtrack_0_2) (`Timeline|Door` :!via `PlayFromStart`)
        (:`Update`
          (bind _returnvalue (+ (`self.Door_Start`) _newtrack_0_2))
          (set `self.Door_End` _returnvalue)
          (`SceneComponent.K2_SetWorldLocation` _cube _returnvalue false false)
          (set `self.Door_Open` true)
          (set `InteractableComponent.InteractionDescriptionText` "Close Door" (`self.Interactable`)))))))

(fn `UserConstructionScript`
  (`InteractableComponent.RegisterTriggerVolume` (`self.Interactable`) (`self.Box`)))