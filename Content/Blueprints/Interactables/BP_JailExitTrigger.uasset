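; BP_JailExitTrigger is an interactable trigger that gates a jail exit door behind a key.
; Its construction script registers TriggerBox with the Interactable component, which starts non-interactable with the unlocked prompt hidden.
; Destruction of the referenced Key actor sets the unlocked state, swaps the locked text for the unlocked text and enables interaction.
; Interacting then destroys the Door actor, hides the text and disables further interaction.
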(event `self.ReceiveBeginPlay`
  (`SceneComponent.SetVisibility` (`self.DoorUnlockedText`) false false)
  (set `InteractableComponent.bCanInteract` false (`self.Interactable`)))

(event `self.Interactable.OnInteractTickBegin`
  (params (_playerCharacter :type "PlayerCharacter Object Reference"))
  ;[1 1 1] On Interact
  (if (`self.IsUnlocked`)
    (set `self.IsOpen` true)
    (`self.K2_DestroyActor` (`self.Door`))
    (`SceneComponent.SetVisibility` (`self.DoorUnlockedText`) false false)
    (set `InteractableComponent.bCanInteract` false (`self.Interactable`))))

(event `self.Key.OnDestroyed`
  (params (DestroyedActor :type "Actor Object Reference"))
  (`SceneComponent.SetVisibility` (`self.DoorLockedText`) false false)
  (`SceneComponent.SetVisibility` (`self.DoorUnlockedText`) true false)
  (set `self.IsUnlocked` true)
  (set `InteractableComponent.bCanInteract` true (`self.Interactable`)))

(fn `UserConstructionScript`
  (`InteractableComponent.RegisterTriggerVolume` (`self.Interactable`) (`self.TriggerBox`)))