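; Prison exit key interactable that serves as a quest objective, completed when the key is picked up.
; Activating its QuestObjective component reveals the ObjectiveMarker, and the pre-pickup event completes the objective.
; On completion it notifies CatastropheMainGameMode, passing the objective and flagging that it does not unlock a new quest.
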(event `self.QuestObjective.OnObjectiveActivate`
  (`SceneComponent.SetVisibility` (`self.ObjectiveMarker`) true false))

(event `self.Receive_PrePickup`
  (`QuestObjectiveComponent.CompleteObjective` (`self.QuestObjective`)))

(event `self.QuestObjective.OnObjectiveComplete`
  (bind _ascatastrophe_main_game_mode (cast `CatastropheMainGameMode` (`GameplayStatics.GetGameMode`)))
  (`CatastropheMainGameMode.OnQuestObjectiveCompletion` _ascatastrophe_main_game_mode (`self.QuestObjective`) false))

(fn `UserConstructionScript`
  (`parent.UserConstructionScript`))