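; BP_LockedDoor is a prison door interactable that stays non-interactable until its referenced Key actor is destroyed.
; Key destruction swaps the locked text for the unlocked text, enables interaction and turns on the door mesh's custom depth.
; A successful interaction through the TriggerBox-registered Interactable then hides the text, disables further interaction, sets Open and calls OpenDoor, which is empty here.
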(event `self.ReceiveBeginPlay`
  (`SceneComponent.SetVisibility` (`self.DoorUnlockedText`) false false)
  (set `InteractableComponent.bCanInteract` false (`self.Interactable`)))

(event `self.Interactable.OnInteractSuccess`
  (params (_playerCharacter :type "PlayerCharacter Object Reference"))
  ;[1 1 1] On Interact
  (if (`self.bUnlocked`)
    (`SceneComponent.SetVisibility` (`self.DoorUnlockedText`) false false)
    (set `InteractableComponent.bCanInteract` false (`self.Interactable`))
    (set `self.bOpen` true)
    (`self.OpenDoor`)))

(event `self.Key.OnDestroyed`
  (params (DestroyedActor :type "Actor Object Reference"))
  (`self.UnlockDoor`))

(fn `OpenDoor`)

(fn `UnlockDoor`
  (`SceneComponent.SetVisibility` (`self.DoorLockedText`) false false)
  (`SceneComponent.SetVisibility` (`self.DoorUnlockedText`) true false)
  (set `self.bUnlocked` true)
  (set `InteractableComponent.bCanInteract` true (`self.Interactable`))
  (`PrimitiveComponent.SetRenderCustomDepth` (`self.DoorMesh`) true))

(fn `UserConstructionScript`
  (`InteractableComponent.RegisterTriggerVolume` (`self.Interactable`) (`self.TriggerBox`)))