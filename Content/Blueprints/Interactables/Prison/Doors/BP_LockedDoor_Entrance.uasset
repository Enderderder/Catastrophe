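; BP_LockedDoor_Entrance is a prison entrance door that blasts apart when its OpenDoor event fires.
; OpenDoor disables collision on the door mesh, then applies damage and an impulse to a destructible mesh from the ExplodeLocation component's position and forward direction.
; It also plays the cave blocker camera shake and switches off custom depth rendering on the destructible.
; The construction script only calls its parent's.
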(event `self.OpenDoor`
  (bind _explodelocation (`self.ExplodeLocation`))
  (`PrimitiveComponent.SetCollisionEnabled` (`self.DoorMesh`) "NoCollision")
  (`DestructibleComponent.ApplyDamage` (`self.DoorDestuctibleMesh`) 5.0 (`SceneComponent.K2_GetComponentLocation` _explodelocation) (`SceneComponent.GetForwardVector` _explodelocation) (`self.ExplodeStrength`))
  (`PlayerCameraManager.PlayCameraShake` :`self` (`GameplayStatics.GetPlayerCameraManager` 0) :`ShakeClass` "/Game/Blueprints/Gameplay/CaveGameplay/BP_CaveBlockerShake.BP_CaveBlockerShake_C")
  (`PrimitiveComponent.SetRenderCustomDepth` (`self.DoorDestuctibleMesh`) false))

(fn `UserConstructionScript`
  (`parent.UserConstructionScript`))