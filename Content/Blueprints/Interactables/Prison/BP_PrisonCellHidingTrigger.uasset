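; A prison cell hiding trigger that serves as a quest objective, playing a cell door cutscene when the player enters it.
; Activating Quest0Objective1 shows the marker and enables the trigger, which starts disabled.
; A tagged player overlap fires once, hiding the marker, disabling input and playing the door-open Level Sequence.
; When the sequence finishes, it completes the objective, restores input and unhides the stunned guard, and completion notifies CatastropheMainGameMode.
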(event `self.ReceiveBeginPlay`
  (`PrimitiveComponent.SetCollisionEnabled` (`self.Trigger`) "NoCollision")
  (`SceneComponent.SetVisibility` (`self.ObjectiveMarker`) false false))

(event `self.Trigger.OnComponentBeginOverlap`
  (params (OverlappedComponent :type "PrimitiveComponent Object Reference") (OtherActor :type "Actor Object Reference") (OtherComp :type "PrimitiveComponent Object Reference") (OtherBodyIndex :type Integer) (bFromSweep :type Boolean) (SweepResult :type "HitResult Structure (by ref)"))
  (if (and (`self.ActorHasTag` OtherActor "Player") (`self.CanHide`))
    (set `self.CanHide` false)
    (bind (_outactor _returnvalue) (`LevelSequencePlayer.CreateLevelSequencePlayer` "/Game/Sequences/S_PrisonCellDoorOpen.S_PrisonCellDoorOpen"))
    (add `MovieSceneSequencePlayer.OnFinished` _returnvalue (delegate `OnCutsceneEnd`))
    (`MovieSceneSequencePlayer.Play` _returnvalue)
    (`SceneComponent.SetVisibility` (`self.ObjectiveMarker`) false false)
    (`self.DisableInput` (`GameplayStatics.GetPlayerCharacter` 0) (`GameplayStatics.GetPlayerController` 0))))

(event `OnCutsceneEnd`
  (`QuestObjectiveComponent.CompleteObjective` (`self.Quest0Objective1`))
  (`self.EnableInput` (`GameplayStatics.GetPlayerCharacter` 0) (`GameplayStatics.GetPlayerController` 0))
  (`self.SetActorHiddenInGame` (`self.StunnedGuard`) false))

(event `self.Quest0Objective1.OnObjectiveActivate`
  (`SceneComponent.SetVisibility` (`self.ObjectiveMarker`) true false)
  (`PrimitiveComponent.SetCollisionEnabled` (`self.Trigger`) "QueryAndPhysics")
  (set `self.CanHide` true))

(event `self.Quest0Objective1.OnObjectiveComplete`
  (bind _ascatastrophe_main_game_mode (cast `CatastropheMainGameMode` (`GameplayStatics.GetGameMode`)))
  (`CatastropheMainGameMode.OnQuestObjectiveCompletion` _ascatastrophe_main_game_mode (`self.Quest0Objective1`) false))

(fn `UserConstructionScript`)