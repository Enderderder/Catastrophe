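; Hideout elevator interactable, bundling its key pickup, gate and moving hatch in one actor.
; Collecting the key removes its mesh and trigger and enables elevator interaction; first entering elevator range adds the key to the player's required-item widget.
; Interacting clears that requirement and slides the gate open via a timeline.
; A player entering the internal trigger lowers the hatch after a short delay, which later snaps back to its origin.
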(event `self.ReceiveBeginPlay`
  (set `self.GateClosedLoc` (`SceneComponent.RelativeLocation` (`self.GateMesh`)))
  (set `self.HatchOriginLoc` (`SceneComponent.K2_GetComponentLocation` (`self.HatchMesh`)))
  (set `InteractableComponent.bCanInteract` false (`self.ElevatorInteract`)))

(event `self.ElevatorInteract.OnInteractSuccess`
  (params (_playerCharacter :type "PlayerCharacter Object Reference"))
  ;[1 1 1] Open gate
  (`/Game/Assets/UI/Widgets/WBP_ItemRequire.RemoveRequiredItem` (`/Game/Blueprints/Characters/Player/BP_PlayerCharacter.RequiredItemWidget` (cast `/Game/Blueprints/Characters/Player/BP_PlayerCharacter` _playerCharacter :!pure true)))
  (bind (_direction _alpha) (`Timeline|OpenElevatorDoorTimeline` :!via `PlayFromStart`)
    (:`Update`
      (`SceneComponent.K2_SetRelativeLocation` (`self.GateMesh`) (`KismetMathLibrary.VLerp` (`self.GateOpenedLoc`) (`self.GateClosedLoc`) _alpha) false false))))

(event `self.ElevatorInteract.OnPlayerEnterInteractRange`
  (params (_playerCharacter :type "PlayerCharacter Object Reference"))
  (if (not (`self.bHasGivenRequire`))
    (`/Game/Assets/UI/Widgets/WBP_ItemRequire.AddRequireItem` (`/Game/Blueprints/Characters/Player/BP_PlayerCharacter.RequiredItemWidget` (cast `/Game/Blueprints/Characters/Player/BP_PlayerCharacter` _playerCharacter :!pure true)) "/Game/Blueprints/Gameplay/Items/BP_Item_ElevatorKey.BP_Item_ElevatorKey_C" 1)
    (set `self.bHasGivenRequire` true)))

(event `self.ElevatorInternalTrigger.OnComponentBeginOverlap`
  (params (OverlappedComponent :type "PrimitiveComponent Object Reference") (OtherActor :type "Actor Object Reference") (OtherComp :type "PrimitiveComponent Object Reference") (OtherBodyIndex :type Integer) (bFromSweep :type Boolean) (SweepResult :type "HitResult Structure (by ref)"))
  ;[1 1 1] Hatch go down
  (if (`self.ActorHasTag` OtherActor "Player")
    (`KismetSystemLibrary.Delay` 1.0)
    (bind (_direction _newtrack_0) (`Timeline|LowerHatchTimeline`)
      (:`Update`
        (`SceneComponent.K2_SetWorldLocation` (`self.HatchMesh`) (+ (`self.HatchOriginLoc`) _newtrack_0) false false))
      (:`Finished`
        (`KismetSystemLibrary.Delay` 2.0)
        (`SceneComponent.K2_SetWorldLocation` (`self.HatchMesh`) (`self.HatchOriginLoc`) false false)))))

(event `self.KeyInteract.OnInteractSuccess`
  (params (_playerCharacter :type "PlayerCharacter Object Reference"))
  ;[1 1 1] Collect key
  (`ActorComponent.K2_DestroyComponent` (`self.KeyMesh`))
  (`ActorComponent.K2_DestroyComponent` (`self.KeyTrigger`))
  (set `InteractableComponent.bCanInteract` true (`self.ElevatorInteract`)))

(fn `UserConstructionScript`
  (`InteractableComponent.RegisterTriggerVolume` (`self.ElevatorInteract`) (`self.ElevatorTrigger`))
  (`InteractableComponent.RegisterTriggerVolume` (`self.KeyInteract`) (`self.KeyTrigger`)))