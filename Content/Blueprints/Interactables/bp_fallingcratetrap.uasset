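; Falling crate trap interactable that moves its body when its trigger box is overlapped.
; BeginPlay caches the body's world location, and any overlap with the box plays a timeline whose track is added to that location each update, without sweeping.
; The trigger box is destroyed on the timeline's first update, so the trap fires only once.
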(event `self.ReceiveBeginPlay`
  (set `self.end` (`SceneComponent.K2_GetComponentLocation` (`self.bodyreference`))))

(event `self.Box.OnComponentBeginOverlap`
  (params (OverlappedComponent :type "PrimitiveComponent Object Reference") (OtherActor :type "Actor Object Reference") (OtherComp :type "PrimitiveComponent Object Reference") (OtherBodyIndex :type Integer) (bFromSweep :type Boolean) (SweepResult :type "HitResult Structure (by ref)"))
  (bind (_direction _newtrack_0) (`Timeline|Timeline_0`)
    (:`Update`
      (`SceneComponent.K2_SetWorldLocation` (`self.bodyreference`) (+ (`self.end`) _newtrack_0) false false)
      (bind _box (`self.Box`)
        (:`then`
          (`ActorComponent.K2_DestroyComponent` _box))
        (:`else`)))))

(fn `UserConstructionScript`)