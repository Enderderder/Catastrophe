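; Tutorial tomato box interactable tied to the second objective of Quest 0, starting unusable with its outline hidden.
; Tick polls that objective, showing the marker only while it is active and enabling the trigger volume's collision and the outline at that point.
; A successful interaction completes the objective unless already completed, as does the PickUpTomato event while it is active.
; Nothing here disables the trigger or outline again afterwards.
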(event `self.ReceiveBeginPlay`
  (`parent.ReceiveBeginPlay`)
  (`self.SetCanUse` false)
  (`SceneComponent.SetVisibility` (`self.OutlineMesh`) false false))

(event `self.ReceiveTick`
  (params (DeltaSeconds :type "Float (single-precision)"))
  (bind _objectivemarker (`self.ObjectiveMarker`))
  (`parent.ReceiveTick` DeltaSeconds)
  (if (`|EnumEquality` (`QuestObjectiveComponent.ObjectiveState` (`self.Quest0Objective2`)) "Active")
    (`SceneComponent.SetVisibility` _objectivemarker true false)
    (`self.SetCanUse` true)
    (`SceneComponent.SetVisibility` (`self.OutlineMesh`) true false)
    (else
      (`SceneComponent.SetVisibility` _objectivemarker false false))))

(event `Receive_PickUpTomato_1`
  (bind _quest0objective2 (`self.Quest0Objective2`))
  (if (`QuestObjectiveComponent.IsObjectiveActive` _quest0objective2)
    (`QuestObjectiveComponent.CompleteObjective` _quest0objective2)))

(event `self.InteractableComponent.OnInteractSuccess`
  (params (_playerCharacter :type "PlayerCharacter Object Reference"))
  (if (not (`|EnumEquality` (`QuestObjectiveComponent.ObjectiveState` (`self.Quest0Objective2`)) "Completed"))
    (`QuestObjectiveComponent.CompleteObjective` (`self.Quest0Objective2`))))

(fn `SetCanUse`
  (params (CanUse :type Boolean))
  (bind _output_get (set `self.CanUse` CanUse))
  (if _output_get
    (`PrimitiveComponent.SetCollisionEnabled` (`self.TriggerVolume`) "QueryAndPhysics")
    (else
      (`PrimitiveComponent.SetCollisionEnabled` (`self.TriggerVolume`) "NoCollision"))))

(fn `UserConstructionScript`
  (`parent.UserConstructionScript`))