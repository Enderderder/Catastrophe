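; BP_WaterFallTrigger is a waterfall trigger that advances quest progress in the game.
; When a Player-tagged actor overlaps its TriggerBox, it completes its QuestObjective through BP_CatastropheMainGameMode and unlocks a new quest.
; A separate LevelTran event, with no caller in this graph, respawns the player at the HUB district's River location.
; It then signals the same objective's completion to CatastropheMainGameMode without unlocking a new quest.
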(event `self.TriggerBox.OnComponentBeginOverlap`
  (params (OverlappedComponent :type "PrimitiveComponent Object Reference") (OtherActor :type "Actor Object Reference") (OtherComp :type "PrimitiveComponent Object Reference") (OtherBodyIndex :type Integer) (bFromSweep :type Boolean) (SweepResult :type "HitResult Structure (by ref)"))
  (if (`self.ActorHasTag` OtherActor "Player")
    (bind _asbp_catastrophe_main_game_mode (cast `/Game/Blueprints/Gameplay/Gamemodes/BP_CatastropheMainGameMode` (`GameplayStatics.GetGameMode`)))
    (`/Game/Blueprints/Gameplay/Gamemodes/BP_CatastropheMainGameMode.CompleteQuestObjective` _asbp_catastrophe_main_game_mode (`self.QuestObjective`) true)))

(event `LevelTran`
  (`RespawnSubsystem.RespawnPlayerAtDistrict` (subsystem `RespawnSubsystem`) "HUB" "River")
  (bind _ascatastrophe_main_game_mode (cast `CatastropheMainGameMode` (`GameplayStatics.GetGameMode`)))
  (`CatastropheMainGameMode.OnQuestObjectiveCompletion` _ascatastrophe_main_game_mode (`self.QuestObjective`) false))

(fn `UserConstructionScript`)