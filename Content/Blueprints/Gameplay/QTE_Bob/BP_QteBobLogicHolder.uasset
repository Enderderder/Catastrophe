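; Logic holder for the QteBob timed-press quick time event, run in slow motion.
; CreateRandomQteBobWith creates the HUD widget, randomizes a success window in the timer's second half, applies time dilation, then arms input after a delay.
; Tick and delay compensate for dilation to keep real-time timing.
; A press or timeout fires OnQteEventComplete with success, miss or timeout, restores normal speed and removes the widget.
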(event `self.ReceiveTick`
  (params (DeltaSeconds :type "Float (single-precision)"))
  (if (`|EnumEquality` (`.EventState_3_0160ABDA4AD465789CEEBB967EDD5B59` (break `/Game/Blueprints/Gameplay/QTE_Bob/FQteEvent` (`self.QteBobEventInfo`))) "NewEnumerator1")
    (`KismetSystemLibrary.PrintString` (`KismetStringLibrary.Concat_StrStr` "QteBob Time: " (`KismetStringLibrary.Conv_DoubleToString` (`self.EventCurrentTime`))) true false (struct :`G` 1.0 :`B` 0.126604 :`A` 1.0) 0.0)
    (bind _output_get (set `self.EventCurrentTime` (+ (`self.EventCurrentTime`) (/ DeltaSeconds (`GameplayStatics.GetGlobalTimeDilation`)))))
    (if (>= _output_get (`.EventDuration_5_B53396794E7A619719A4F38B54CD07D7` (break `/Game/Blueprints/Gameplay/QTE_Bob/FQteEvent` (`self.QteBobEventInfo`))))
      (setmembers `/Game/Blueprints/Gameplay/QTE_Bob/FQteEvent` :`StructRef` (`self.QteBobEventInfo`) :`EventState` "NewEnumerator3")
      (`self.OnQteEventComplete` "FailedByTimeOut")
      (`KismetSystemLibrary.PrintString` "QteBob: TimeOut!" true false (struct :`G` 1.0 :`B` 0.470018 :`A` 1.0) 5.0)
      (`GameplayStatics.SetGlobalTimeDilation` 1.0)
      (`self.RemoveWidget`))))

(event `InputAction|Qte`
  (params (Key :type "Key Structure"))
  (bind ((`EventDuration_5_B53396794E7A619719A4F38B54CD07D7` _eventduration) (`SuccessAreaRange_10_830E207C47C037A985FA5F969760BFDE` _successarearange) (`SuccessAreaStart_9_5D43AE07460CF26E26165CBD09CB79F6` _successareastart)) (break `/Game/Blueprints/Gameplay/QTE_Bob/FQteEvent` (`self.QteBobEventInfo`)))
  (bind ((`EventDuration_5_B53396794E7A619719A4F38B54CD07D7` _eventduration_2) (`SuccessAreaStart_9_5D43AE07460CF26E26165CBD09CB79F6` _successareastart_2)) (break `/Game/Blueprints/Gameplay/QTE_Bob/FQteEvent` (`self.QteBobEventInfo`)))
  (:`Pressed`
    (if (`|EnumEquality` (`.EventState_3_0160ABDA4AD465789CEEBB967EDD5B59` (break `/Game/Blueprints/Gameplay/QTE_Bob/FQteEvent` (`self.QteBobEventInfo`))) "NewEnumerator1")
      (if (and (>= (`self.EventCurrentTime`) (* _eventduration_2 (/ _successareastart_2 100.0))) (<= (`self.EventCurrentTime`) (* _eventduration (/ (+ _successarearange _successareastart) 100.0))))
        (setmembers `/Game/Blueprints/Gameplay/QTE_Bob/FQteEvent` :`StructRef` (`self.QteBobEventInfo`) :`EventState` "NewEnumerator2")
        (`self.OnQteEventComplete` "Success")
        (`KismetSystemLibrary.PrintString` "QteBob: Success!" true false (struct :`G` 1.0 :`B` 0.470018 :`A` 1.0) 5.0)
        (else
          (setmembers `/Game/Blueprints/Gameplay/QTE_Bob/FQteEvent` :`StructRef` (`self.QteBobEventInfo`) :`EventState` "NewEnumerator4")
          (`self.OnQteEventComplete` "FailedByMissHit")
          (`KismetSystemLibrary.PrintString` "QteBob: Failed!" true false (struct :`G` 1.0 :`B` 0.470018 :`A` 1.0) 5.0)))
      (`GameplayStatics.SetGlobalTimeDilation` 1.0)
      (`self.RemoveWidget`))))

(event `CreateRandomQteBobWith`
  (params (Range :type "Float (double-precision)" :default 20.0))
  (bind _returnvalue (`KismetMathLibrary.FMin` Range 50.0))
  (bind _asbp_player_character (cast `/Game/Blueprints/Characters/BP_PlayerCharacter` (`GameplayStatics.GetPlayerCharacter` 0)))
  (`|ExecutionSequence`
    (:`then_0`
      (bind _qtebobwidget (`/Game/Assets/UI/Widgets/WBP_HUD.CreateQteBobWidget` (cast `/Game/Assets/UI/Widgets/WBP_HUD` (`PlayerCharacter.PlayerWidget` _asbp_player_character) :!pure true) self null null))
      (set `self.QteBobWidgert` _qtebobwidget))
    (:`then_1`
      (set `self.QteBobEventInfo` (make `/Game/Blueprints/Gameplay/QTE_Bob/FQteEvent` "NewEnumerator0" 1.0 _returnvalue (`KismetMathLibrary.RandomFloatInRange` 50.0 (- 100.0 _returnvalue))))
      (bind _qtebobwidgert (`self.QteBobWidgert`)
        (:`then`
          (`/Game/Assets/UI/Widgets/WBP_Qte.InitiateQteUI` _qtebobwidgert)
          (`GameplayStatics.SetGlobalTimeDilation` (`self.EventDilation`))
          (`KismetSystemLibrary.Delay` (* 1.0 (`GameplayStatics.GetGlobalTimeDilation`)))
          (bind _structout (setmembers `/Game/Blueprints/Gameplay/QTE_Bob/FQteEvent` :`StructRef` (`self.QteBobEventInfo`) :`EventState` "NewEnumerator1"))
          (`KismetSystemLibrary.PrintString` (`KismetStringLibrary.Concat_StrStr` "Qte Starting Time: " (`KismetStringLibrary.Conv_DoubleToString` (* (`.EventDuration_5_B53396794E7A619719A4F38B54CD07D7` (break `/Game/Blueprints/Gameplay/QTE_Bob/FQteEvent` _structout)) (/ (`.SuccessAreaStart_9_5D43AE07460CF26E26165CBD09CB79F6` (break `/Game/Blueprints/Gameplay/QTE_Bob/FQteEvent` _structout)) 100.0)))) true false (struct :`G` 1.0 :`B` 0.687033 :`A` 1.0) 5.0)
          (`self.EnableInput` (`GameplayStatics.GetPlayerController` 0)))
        (:`else`)))))

(event `RemoveWidget`
  ;[1 1 1] Remove the QTE widget
  (`Widget.RemoveFromParent` (`self.QteBobWidgert`)))

(fn `UserConstructionScript`)