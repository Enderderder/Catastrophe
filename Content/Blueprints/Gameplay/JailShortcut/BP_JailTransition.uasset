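; Jail shortcut actor that gates a pipe transition to the HUB district's River behind moving a rock.
; Interacting with the rock plays a level sequence with the player hidden, enables a door blocker, then outlines the drain via custom depth after a fixed delay.
; The pipe respawns the player through the respawn subsystem and moves them to RockSpawn, or briefly shows a blocked-cell widget if the rock remains.
; An older S_RockPush sequence path is left unconnected.
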(event `self.InteractableRock.OnInteractSuccess`
  (params (_playerCharacter :type "PlayerCharacter Object Reference"))
  (bind _jaildoorblock (`self.JailDoorBlock`))
  (`self.SetActorHiddenInGame` _playerCharacter true)
  (set `self.bRockRemoved` true)
  (bind (_outactor _returnvalue) (`LevelSequencePlayer.CreateLevelSequencePlayer` "/Game/Sequences/MoveRock.MoveRock"))
  (`MovieSceneSequencePlayer.Play` _returnvalue)
  (`SceneComponent.SetHiddenInGame` _jaildoorblock false false)
  (`PrimitiveComponent.SetCollisionEnabled` _jaildoorblock "QueryAndPhysics")
  (`KismetSystemLibrary.Delay` 7.16)
  (`self.SetActorHiddenInGame` _playerCharacter false)
  (`PrimitiveComponent.SetRenderCustomDepth` (`self.Drain`) true)
  (set `InteractableComponent.bCanInteract` false (`self.InteractableRock`)))

(event `OnRemoveDoorFinished`
  (`self.EnableInput` (`GameplayStatics.GetPlayerController` 0))
  (`self.SetActorHiddenInGame` (`GameplayStatics.GetPlayerCharacter` 0) false)
  (set `self.bRockRemoved` true))

(event `self.InteractablePipe.OnInteractSuccess`
  (params (_playerCharacter :type "PlayerCharacter Object Reference"))
  (if (`self.bRockRemoved`)
    (`RespawnSubsystem.RespawnPlayerAtDistrict` (subsystem `RespawnSubsystem`) "HUB" "River")
    (`self.K2_SetActorTransform` _playerCharacter (`KismetMathLibrary.Conv_VectorToTransform` (`SceneComponent.K2_GetComponentLocation` (`self.RockSpawn`))) false false)
    (else
      (bind _returnvalue (`|CreateWidget` "/Game/Assets/UI/Widgets/WBP_CellBlock.WBP_CellBlock_C"))
      (bind _output_get (set `self.NopeWidget` _returnvalue))
      (`UserWidget.AddToViewport` _output_get 0)
      (`KismetSystemLibrary.Delay` 3.0)
      (`Widget.RemoveFromParent` (`self.NopeWidget`)))))

(fn `UserConstructionScript`
  (`parent.UserConstructionScript`)
  (`InteractableComponent.RegisterTriggerVolume` (`self.InteractableRock`) (`self.Rock`))
  (`InteractableComponent.RegisterTriggerVolume` (`self.InteractablePipe`) (`self.Cell`)))