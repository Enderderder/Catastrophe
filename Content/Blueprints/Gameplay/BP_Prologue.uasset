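; BP_Prologue is an actor that shows the game's prologue as an image sequence on screen.
; On BeginPlay it creates a WBP_Prologue widget and adds it to the viewport at a high Z-order.
; Each U key press advances the widget's image until a counter reaches its maximum, and the next press destroys the actor.
; EndPlay then removes the widget from the screen.
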(event `self.ReceiveBeginPlay`
  (bind _returnvalue (`|CreateWidget` "/Game/Assets/UI/Widgets/WBP_Prologue.WBP_Prologue_C" (`GameplayStatics.GetPlayerController` 0)))
  (bind _output_get (set `self.PrologueWidget` _returnvalue))
  (`UserWidget.AddToViewport` _output_get 1000))

(event `Key|U`
  (params (Key :type "Key Structure"))
  (:`Pressed`
    (if (>= (`self.IncrementedTime`) (`self.MaxIncrementTime`))
      (`self.K2_DestroyActor`)
      (else
        (`/Game/Assets/UI/Widgets/WBP_Prologue.IncrementImage` (`self.PrologueWidget`))
        (`/Engine/EditorBlueprintResources/StandardMacros.IncrementInt` (`self.IncrementedTime`))))))

(event `self.ReceiveEndPlay`
  (params (EndPlayReason :type "EEndPlayReason Enum" :default "Destroyed"))
  (`Widget.RemoveFromParent` (`self.PrologueWidget`)))

(fn `UserConstructionScript`)