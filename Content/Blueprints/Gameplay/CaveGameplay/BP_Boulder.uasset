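; BP_Boulder is a cave gameplay boulder that falls and turns on its block collision when a quick-time event succeeds.
; A player-tagged overlap spawns a BP_QteBobLogicHolder, starts a random bob QTE and disables the trigger, making it one-shot.
; On success, BlockCollision, disabled at BeginPlay, becomes query-only and the mesh's ABP_FallingCrate anim instance gets its Fallen flag set.
; Both failure outcomes only print a debug string.
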(event `self.ReceiveBeginPlay`
  (`PrimitiveComponent.SetCollisionEnabled` (`self.BlockCollision`) "NoCollision"))

(event `self.QteTriggerCollison.OnComponentBeginOverlap`
  (params (OverlappedComponent :type "PrimitiveComponent Object Reference") (OtherActor :type "Actor Object Reference") (OtherComp :type "PrimitiveComponent Object Reference") (OtherBodyIndex :type Integer) (bFromSweep :type Boolean) (SweepResult :type "HitResult Structure (by ref)"))
  (if (`self.ActorHasTag` OtherActor "Player")
    (bind _returnvalue (`|SpawnActorFromClass` "/Game/Blueprints/Gameplay/QTE_Bob/BP_QteBobLogicHolder.BP_QteBobLogicHolder_C" (`KismetMathLibrary.MakeTransform` (0.0 0.0 0.0)) "AlwaysSpawn" "OverrideRootScale" null null))
    (bind _output_get (set `self.QteHolder` _returnvalue))
    (`/Game/Blueprints/Gameplay/QTE_Bob/BP_QteBobLogicHolder.CreateRandomQteBobWith` _output_get 30.0)
    (add `QteBobLogicHolder.OnQteEventComplete` _output_get (delegate `OnQteComplete`))
    (`PrimitiveComponent.SetCollisionEnabled` (`self.QteTriggerCollison`) "NoCollision")))

(event `OnQteComplete`
  (params (_eventState :type "EQteEventState Enum" :default "None"))
  (switch `EQteEventState` _eventState
    (:`Success`
      (`PrimitiveComponent.SetCollisionEnabled` (`self.BlockCollision`) "QueryOnly")
      (set `/Game/Assets/Kitsets/Kitset_Market/FallingCrates/ABP_FallingCrate.bFallen` true (cast `/Game/Assets/Kitsets/Kitset_Market/FallingCrates/ABP_FallingCrate` (`SkeletalMeshComponent.GetAnimInstance` (`self.BoulderMesh`)) :!pure true)))
    (:`FailedByTimeOut`
      (`KismetSystemLibrary.PrintString` "NUTTIN HAPPEN" :!label _label))
    (:`FailedByMissHit`
      (goto _label))))

(fn `UserConstructionScript`)