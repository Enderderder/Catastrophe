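; BP_CaveBlocker is a rock obstacle in the cave gameplay that shatters when an actor tagged Caterpillar overlaps it.
; A one-shot overlap on the destructible mesh calls SmashRock, which disables the separate blocking mesh's collision and applies damage with an impulse.
; The impulse points from the impact point toward the blocker's origin, and the actor despawns after a set lifespan.
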(event `self.RockDestructableMesh.OnComponentBeginOverlap`
  (params (OverlappedComponent :type "PrimitiveComponent Object Reference") (OtherActor :type "Actor Object Reference") (OtherComp :type "PrimitiveComponent Object Reference") (OtherBodyIndex :type Integer) (bFromSweep :type Boolean) (SweepResult :type "HitResult Structure (by ref)"))
  (bind (_bblockinghit _binitialoverlap _time _distance _location _impactpoint) (`GameplayStatics.BreakHitResult` SweepResult))
  (if (`self.bHasExploded`)
    _
    (elif (`self.ActorHasTag` OtherActor "Caterpillar")
      (set `self.bHasExploded` true)
      (`self.SmashRock` _impactpoint (`KismetMathLibrary.Normal` (- (`self.K2_GetActorLocation`) _impactpoint)))
      (`self.SetLifeSpan` (`self.DespawnTime`)))))

(fn `SmashRock`
  (params (ImpactLocation :type "Vector Structure") (ImpactDirection :type "Vector Structure"))
  (`PrimitiveComponent.SetCollisionEnabled` (`self.BlockingMesh`) "NoCollision")
  (`DestructibleComponent.ApplyDamage` (`self.RockDestructableMesh`) 2.0 ImpactLocation ImpactDirection (`self.ExplodeStrength`)))

(fn `UserConstructionScript`)