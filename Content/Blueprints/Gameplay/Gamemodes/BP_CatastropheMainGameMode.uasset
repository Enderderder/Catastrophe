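; Main game mode for Catastrophe that spawns a tutorial bubble on BeginPlay and provides events for jail reloading and quick-time events.
; ReloadJail unloads the ChrisJail stream level and requests it again through the respawn subsystem as a jail district.
; QteBobEvent spawns a QTE Bob logic holder actor and has it create a random ranged QTE.
; The CreateQteBobEvent graph holds only disconnected slow-motion QTE logic that never runs.
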(event `self.ReceiveBeginPlay`
  ;[1 1 1] Force tutorial spawn
  (bind _returnvalue (`|SpawnActorFromClass` "/Game/Blueprints/Gameplay/Tutorial/BP_TutorialBubble.BP_TutorialBubble_C" (`KismetMathLibrary.MakeTransform` (0.0 0.0 0.0)) "AlwaysSpawn" "OverrideRootScale" null null))
  (set `self.TutorialBubble` _returnvalue))

(event `ReloadJail`
  (`GameplayStatics.UnloadStreamLevel` "ChrisJail")
  (`RespawnSubsystem.LoadLevelStreaming` (subsystem `RespawnSubsystem`) (make `LoadStreamingLevelInfo` "DefaultName" "ChrisJail" false true "JAIL")))

(event `QteBobEvent`
  (bind _returnvalue (`|SpawnActorFromClass` "/Game/Blueprints/Gameplay/QTE_Bob/BP_QteBobLogicHolder.BP_QteBobLogicHolder_C" (`KismetMathLibrary.MakeTransform` (0.0 0.0 0.0)) "AlwaysSpawn" "OverrideRootScale" null null))
  (bind _output_get (set `self.QteBobLogicActor` _returnvalue))
  (`/Game/Blueprints/Gameplay/QTE_Bob/BP_QteBobLogicHolder.CreateRandomQteBobWithRange` _output_get 10.0))

(fn `UserConstructionScript`)