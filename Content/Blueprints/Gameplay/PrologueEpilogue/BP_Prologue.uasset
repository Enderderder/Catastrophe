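; Prologue actor that shows a full-screen, key-driven scrolling image sequence through the WBP_PrologueEpilogue widget.
; BeginPlay adds the widget at high Z-order, and Space, S or Down step a counter forward while W or Up step it back.
; Each step sends the counter and increment size to the widget's scroll.
; Advancing past the maximum destroys the actor, fires OnLogueFinish, and EndPlay removes the widget.
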(event `self.ReceiveBeginPlay`
  (bind _returnvalue (`|CreateWidget` "/Game/Assets/UI/Widgets/PrologueEpilogue/WBP_PrologueEpilogue.WBP_PrologueEpilogue_C" (`GameplayStatics.GetPlayerController` 0)))
  (bind _output_get (set `self.PrologueWidget` _returnvalue))
  (`UserWidget.AddToViewport` _output_get 1000))

(event `Key|SpaceBar`
  (params (Key :type "Key Structure"))
  (:`Pressed`
    (if (>= (`self.IncrementedTime`) (`self.MaxIncrementTime`)) :!label _label
      (`self.K2_DestroyActor`)
      (`self.OnLogueFinish`)
      (else
        (`/Engine/EditorBlueprintResources/StandardMacros.IncrementInt` (`self.IncrementedTime`)
          (:`  `
            (`/Game/Assets/UI/Widgets/PrologueEpilogue/WBP_PrologueEpilogue.SetImageScroll` (`self.PrologueWidget`) (`self.IncrementedTime`) (`self.IncrementSize`) :!label _label_2)))))))

(event `Key|S`
  (params (Key :type "Key Structure"))
  (:`Pressed`
    (goto _label)))

(event `Key|Down`
  (params (Key :type "Key Structure"))
  (:`Pressed`
    (goto _label)))

(event `Key|W`
  (params (Key :type "Key Structure"))
  (:`Pressed`
    (if (> (`self.IncrementedTime`) 0) :!label _label_3
      (`/Engine/EditorBlueprintResources/StandardMacros.DecrementInt` (`self.IncrementedTime`)
        (:`  `
          (goto _label_2))))))

(event `Key|Up`
  (params (Key :type "Key Structure"))
  (:`Pressed`
    (goto _label_3)))

(event `self.ReceiveEndPlay`
  (params (EndPlayReason :type "EEndPlayReason Enum" :default "Destroyed"))
  (`Widget.RemoveFromParent` (`self.PrologueWidget`)))

(fn `UserConstructionScript`)