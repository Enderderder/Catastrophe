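; Brewing machine for BigFluff gameplay that produces a catnip ball pickup when brewing is triggered.
; Brewing plays the activation montage on the machine mesh, waits out its duration, then spawns the catnip pickup class at the pickup point.
; When a player enters the interactable component's range, it adds a required-item entry to that player's widget, with the amount set to zero.
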(event `self.Receive_OnBrewing`
  (bind _returnvalue (`AnimInstance.Montage_Play` (`SkeletalMeshComponent.GetAnimInstance` (`self.BrewingMachineMesh`)) "/Game/Assets/BrewingMachine/Animations/AM_BrewingMachine_Activate.AM_BrewingMachine_Activate" 1.0 "Duration" 0.0 true))
  (`KismetSystemLibrary.Delay` _returnvalue)
  (bind _returnvalue_2 (`|SpawnActorFromClass` (`self.CatnipPickupClass`) (`SceneComponent.K2_GetComponentToWorld` (`self.CatnipBallPickupPoint`)) "AdjustIfPossibleButAlwaysSpawn" "OverrideRootScale" null null))
  (cast `/Game/Blueprints/Interactables/BP_CatnipBallPickup` _returnvalue_2))

(event `self.InteractableComponent.OnPlayerEnterInteractRange`
  (params (_playerCharacter :type "PlayerCharacter Object Reference"))
  (bind _asbp_player_character (cast `/Game/Blueprints/Characters/Player/BP_PlayerCharacter` _playerCharacter))
  (bind _requireditemwidget (`/Game/Blueprints/Characters/Player/BP_PlayerCharacter.RequiredItemWidget` _asbp_player_character)
    (:`then`
      (`/Game/Assets/UI/Widgets/RequireItemUi/WBP_ItemRequire.AddRequireItem` _requireditemwidget null 0))
    (:`else`)))

(fn `UserConstructionScript`)