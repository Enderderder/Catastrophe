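; BP_ItemCrate is an interactable crate that puts an item into the player's backpack.
; Its construction script registers the Trigger volume with the Interactable component.
; On a successful interaction with a valid GiveItemClass, it spawns a temporary item actor, passes it to the BackPackComponent's InsertItem, then destroys that actor.
; The crate is hidden with collision disabled afterwards rather than destroyed.
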(event `self.Interactable.OnInteractSuccess`
  (params (_playerCharacter :type "PlayerCharacter Object Reference"))
  (bind _giveitemclass (`self.GiveItemClass`)
    (:`then`
      (bind _returnvalue (`|SpawnActorFromClass` _giveitemclass (`KismetMathLibrary.MakeTransform` (0.0 0.0 0.0)) "AlwaysSpawn" "OverrideRootScale" null null))
      (`BackPackComponent.InsertItem` (`PlayerCharacter.BackPackComponent` _playerCharacter) _returnvalue)
      (`self.SetActorHiddenInGame` true)
      (`self.SetActorEnableCollision` false)
      (`self.K2_DestroyActor` _returnvalue))
    (:`else`)))

(fn `UserConstructionScript`
  (`InteractableComponent.RegisterTriggerVolume` (`self.Interactable`) (`self.Trigger`)))