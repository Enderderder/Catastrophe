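; Interactable chest actor that acts as a quest target for two quest objectives.
; On interact, it completes the first objective if that one is active, otherwise the second if that one is active, so each interaction completes at most one.
; Both objective components print debug messages when they activate and complete.
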(event `self.InteractableCompoenent.OnInteract`
  (params (_playerCharacter :type "PlayerCharacter Object Reference"))
  (if (`|EnumEquality` (`QuestObjectiveComponent.ObjectiveState` (`self.QuestObjective1`)) "Active")
    (`QuestObjectiveComponent.CompleteObjective` (`self.QuestObjective1`))
    (elif (`|EnumEquality` (`QuestObjectiveComponent.ObjectiveState` (`self.QuestObjective2`)) "Active")
      (`QuestObjectiveComponent.CompleteObjective` (`self.QuestObjective2`)))))

(event `self.QuestObjective1.OnObjectiveActivate`
  (`KismetSystemLibrary.PrintString` "Objective (1) Activated!" true true (struct :`G` 0.66 :`B` 1.0 :`A` 1.0) 5.0))

(event `self.QuestObjective1.OnObjectiveComplete`
  (`KismetSystemLibrary.PrintString` "Objective (1) Complete!" true true (struct :`G` 0.66 :`B` 1.0 :`A` 1.0) 5.0))

(event `self.QuestObjective2.OnObjectiveActivate`
  (`KismetSystemLibrary.PrintString` "Objective (2) Activated!" true true (struct :`G` 0.66 :`B` 1.0 :`A` 1.0) 5.0))

(event `self.QuestObjective2.OnObjectiveComplete`
  (`KismetSystemLibrary.PrintString` "Objective (2) Complete!" true true (struct :`G` 0.66 :`B` 1.0 :`A` 1.0) 5.0))

(fn `UserConstructionScript`)