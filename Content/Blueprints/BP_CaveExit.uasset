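; BP_CaveExit is an interactable cave exit that plays the S_EtoT cutscene when a player successfully interacts with it.
; On BeginPlay it fills WayPointArray with three waypoints intended for climbing.
; Interaction enables the player's T-pose state, starts the cutscene through BP_CatastropheMainGameMode and disables further interaction.
; The cutscene's finished callback turns the T-pose state off again.
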(event `self.ReceiveBeginPlay`
  (bind _waypointarray (`self.WayPointArray`))
  ;[1 1 1] Setup the array of way point  for climbing
  (`KismetArrayLibrary.Array_Clear` _waypointarray)
  (`KismetArrayLibrary.Array_Append` _waypointarray (`|MakeArray` (`self.WayPoint_1`) (`self.WayPoint_2`) (`self.WayPoint_3`))))

(event `self.InteractableComponent.OnInteractSuccess`
  (params (_playerCharacter :type "PlayerCharacter Object Reference"))
  (`PlayerCharacter.SetPlayerTPoseEable` _playerCharacter true)
  (bind _return_value (`/Game/Blueprints/Gameplay/Gamemodes/BP_CatastropheMainGameMode.PlayCutscene` :`self` (cast `/Game/Blueprints/Gameplay/Gamemodes/BP_CatastropheMainGameMode` (`GameplayStatics.GetGameMode`) :!pure true) :`Cutscene` "/Game/Sequences/S_EtoT.S_EtoT"))
  (add `MovieSceneSequencePlayer.OnFinished` _return_value (delegate `OnCutsceneFinished`))
  (set `InteractableComponent.bCanInteract` false (`self.InteractableComponent`)))

(event `OnCutsceneFinished`
  (`PlayerCharacter.SetPlayerTPoseEable` (stale `self.InteractableComponent.OnInteractSuccess` _playerCharacter) false))

(fn `UserConstructionScript`
  (`parent.UserConstructionScript`))