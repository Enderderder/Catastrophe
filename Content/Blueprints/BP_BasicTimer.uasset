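; BP_BasicTimer is a countdown timer that locks the holding cell exit door when time runs out.
; It shows a WBP_Timer widget from BeginPlay until EndPlay.
; A Delay on Tick decrements TimeSec about once per second.
; At zero or below, it calls LockDoor on the first BP_HoldingCellExitDoor found, repeating each second, then casts to the game mode without using the result.
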(event `self.ReceiveBeginPlay`
  ;[1 1 1] Event BeginPlay
  (bind _returnvalue (`|CreateWidget` "/Game/Assets/UI/Widgets/WBP_Timer.WBP_Timer_C"))
  (bind _output_get (set `self.TimerWidget` _returnvalue))
  (`UserWidget.AddToViewport` _output_get 0))

(event `self.ReceiveTick`
  (params (DeltaSeconds :type "Float (single-precision)"))
  ;[1 1 1] Event Tick
  (`KismetSystemLibrary.Delay` 1.0)
  (bind _output_get (set `self.TimeSec` (- (`self.TimeSec`) 1)))
  (if (<= _output_get 0)
    (bind _outactors (`GameplayStatics.GetAllActorsOfClass` "/Game/Blueprints/Gameplay/LevelStreaming/BP_HoldingCellExitDoor.BP_HoldingCellExitDoor_C"))
    (`/Game/Blueprints/Gameplay/LevelStreaming/BP_HoldingCellExitDoor.LockDoor` (`|GetArrayItem` _outactors))
    (cast `/Game/Blueprints/Gameplay/Gamemodes/BP_CatastropheMainGameMode` (`GameplayStatics.GetGameMode`))))

(event `self.ReceiveEndPlay`
  (params (EndPlayReason :type "EEndPlayReason Enum" :default "Destroyed"))
  ;[1 1 1] Event Tick
  (`Widget.RemoveFromParent` (`self.TimerWidget`)))

(fn `UserConstructionScript`)