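; BP_MarketFish is a pickup item, a market fish that serves as the second objective of Quest 1.
; The pre-pickup event completes Quest1Objective2 if that objective is active.
; When the objective activates, it updates the player's quest widget after a validity check.
; Tick and construction only call the parent, and the objective-complete handler is empty.
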(event `self.ReceiveTick`
  (params (DeltaSeconds :type "Float (single-precision)"))
  (`parent.ReceiveTick` DeltaSeconds))

(event `self.Receive_PrePickup`
  (if (`|EnumEquality` (`QuestObjectiveComponent.ObjectiveState` (`self.Quest1Objective2`)) "Active")
    (`QuestObjectiveComponent.CompleteObjective` (`self.Quest1Objective2`))))

(event `self.Quest1Objective2.OnObjectiveActivate`
  (bind _questwidget (`/Game/Blueprints/Characters/BP_PlayerCharacter.QuestWidget` (`self.PlayerReference`))
    (:`then`
      (`/Game/Assets/UI/Widgets/Quests/WBP_QuestUnlocked.Update` _questwidget (`self.Quest1Objective2`)))
    (:`else`)))

(event `self.Quest1Objective2.OnObjectiveComplete`)

(fn `UserConstructionScript`
  (`parent.UserConstructionScript`))