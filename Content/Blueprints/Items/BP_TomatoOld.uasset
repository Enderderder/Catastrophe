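; Tomato projectile actor, apparently an older version, that splats on whatever it hits.
; On BeginPlay it predicts its path from the ProjectileMovement velocity without collision tracing and draws it as persistent debug.
; When the mesh hits, it spawns a short-lived splat decal aligned to the impact normal, plays an attenuated splat sound and destroys itself.
; A forward AddImpulse launch on the mesh is left unconnected and never runs.
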(event `self.ReceiveBeginPlay`
  (`GameplayStatics.Blueprint_PredictProjectilePath_Advanced` (make `PredictProjectilePathParams` (`self.K2_GetActorLocation`) (`MovementComponent.Velocity` (`self.ProjectileMovement`)) false (`.SphereRadius` (`KismetSystemLibrary.GetComponentBounds` (`self.TomatoMesh`))) 1.0 true "ECC_WorldStatic" (`|MakeArray` "ObjectTypeQuery4" :!type "EObjectTypeQuery Enum") (`|MakeArray` (`GameplayStatics.GetPlayerCharacter` 0) :!type "Actor Object Reference") 20.0 0.0 "Persistent" 1.0 true)))

(event `self.TomatoMesh.OnComponentHit`
  (params (HitComponent :type "PrimitiveComponent Object Reference") (OtherActor :type "Actor Object Reference") (OtherComp :type "PrimitiveComponent Object Reference") (NormalImpulse :type "Vector Structure") (Hit :type "HitResult Structure (by ref)"))
  (`GameplayStatics.SpawnDecalAtLocation` "/Game/Assets/Stall_Fruit/M_TomatoSplat_Decal.M_TomatoSplat_Decal" (50.0 50.0 50.0) (`SceneComponent.K2_GetComponentLocation` (`self.TomatoMesh`)) (`KismetMathLibrary.MakeRotationFromAxes` (`.ImpactNormal` (`GameplayStatics.BreakHitResult` Hit))) 5.0)
  (`GameplayStatics.PlaySoundAtLocation` "/Game/Sound/Audio_TomatoSplat.Audio_TomatoSplat" (`SceneComponent.K2_GetComponentLocation` (`self.TomatoMesh`)) (struct) 1.0 1.0 0.0 "/Game/Assets/Attenuation/ATT_Splash.ATT_Splash" null null)
  (`self.K2_DestroyActor`))

(fn `UserConstructionScript`)