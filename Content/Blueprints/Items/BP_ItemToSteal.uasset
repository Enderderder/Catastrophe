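; BP_ItemToSteal is a stealable pickup item that shows an interaction prompt when the player is near.
; Its Trigger overlap shows the text for the player while IsUsable is set, and Tick turns it toward the camera.
; RecievePickUpItem simply destroys the actor.
; Disconnected leftover logic for hiding the item, showing a carried fish and slowing the player never runs, and the cached PlayerReference is unused.
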(event `self.ReceiveBeginPlay`
  (`SceneComponent.SetVisibility` (`self.InteractionText`) false false)
  (bind _asbp_player_character (cast `/Game/Blueprints/Characters/BP_PlayerCharacter` (`GameplayStatics.GetPlayerCharacter` 0)))
  (set `self.PlayerReference` _asbp_player_character))

(event `self.ReceiveTick`
  (params (DeltaSeconds :type "Float (single-precision)"))
  (bind _interactiontext (`self.InteractionText`))
  (if (`SceneComponent.IsVisible` _interactiontext)
    (`SceneComponent.K2_SetWorldRotation` (`self.InteractionText`) (`KismetMathLibrary.FindLookAtRotation` (`SceneComponent.K2_GetComponentLocation` _interactiontext) (`PlayerCameraManager.GetCameraLocation` (`PlayerController.PlayerCameraManager` (`GameplayStatics.GetPlayerController` 0)))) false false)))

(event `self.Trigger.OnComponentBeginOverlap`
  (params (OverlappedComponent :type "PrimitiveComponent Object Reference") (OtherActor :type "Actor Object Reference") (OtherComp :type "PrimitiveComponent Object Reference") (OtherBodyIndex :type Integer) (bFromSweep :type Boolean) (SweepResult :type "HitResult Structure (by ref)"))
  (if (and (== OtherActor (`GameplayStatics.GetPlayerCharacter` 0)) (`self.isUsable`))
    (`SceneComponent.SetVisibility` (`self.InteractionText`) true false)))

(event `self.Trigger.OnComponentEndOverlap`
  (params (OverlappedComponent :type "PrimitiveComponent Object Reference") (OtherActor :type "Actor Object Reference") (OtherComp :type "PrimitiveComponent Object Reference") (OtherBodyIndex :type Integer))
  (if (== OtherActor (`GameplayStatics.GetPlayerCharacter` 0))
    (`SceneComponent.SetVisibility` (`self.InteractionText`) false false)))

(event `Key|E`
  (params (Key :type "Key Structure")))

(event `self.Recieve_PickUpItem`
  ;[1 1 1] OnPickup
  (`self.K2_DestroyActor`))

(fn `UserConstructionScript`)