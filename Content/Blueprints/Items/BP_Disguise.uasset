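; BP_Disguise is a disguise item actor with a mesh and a world-space timer widget.
; On BeginPlay it hands itself to the WBP_DisguiseTimer widget and places the disguise mesh 150 units above the actor's location.
; Each Tick it turns the timer widget to face the player character's follow camera.
; The use and end disguise events are empty here.
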(event `self.ReceiveBeginPlay`
  (bind (_returnvalue_x _returnvalue_y _returnvalue_z) (`KismetMathLibrary.BreakVector` (`self.K2_GetActorLocation`)))
  (bind _aswbp_disguise_timer (cast `/Game/Assets/UI/Widgets/WBP_DisguiseTimer` (`WidgetComponent.GetUserWidgetObject` (`self.TimerWidget`))))
  (set `/Game/Assets/UI/Widgets/WBP_DisguiseTimer.Disguise` self _aswbp_disguise_timer)
  (`SceneComponent.K2_SetWorldLocation` (`self.DisguiseMesh`) (`KismetMathLibrary.MakeVector` _returnvalue_x _returnvalue_y (- _returnvalue_z -150.0)) false false))

(event `self.ReceiveTick`
  (params (DeltaSeconds :type "Float (single-precision)"))
  (bind _asbp_player_character (cast `/Game/Blueprints/Characters/Player/BP_PlayerCharacter` (`GameplayStatics.GetPlayerCharacter` 0)))
  (`SceneComponent.K2_SetWorldRotation` (`self.TimerWidget`) (`KismetMathLibrary.FindLookAtRotation` (`SceneComponent.K2_GetComponentLocation` (`self.TimerWidget`)) (`SceneComponent.K2_GetComponentLocation` (`PlayerCharacter.FollowCamera` _asbp_player_character))) false false))

(event `self.Receive_OnUseDisguise`)

(event `self.Receive_OnEndDisguise`)

(fn `UserConstructionScript`)